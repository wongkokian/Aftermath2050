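; BP_Table is a table actor under the fruit weapons folder that presents a random assortment of six trays.
; Its Construction Script gives each of the six Tray child actor components a class picked independently at random from the FruitParty array, so duplicates can occur.
; The selection is unseeded, so it rerolls whenever construction reruns, and the event graph holds no active logic.
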(event EventBeginPlay)

(event Collision|EventActorBeginOverlap
  (params (OtherActor :type Actor%20Object%20Reference)))

(event EventTick
  (params (DeltaSeconds :type Float%20%28single-precision%29)))

(fn ConstructionScript
  (bind _fruit_party (Variables|Default|GetFruit%20party))
  (bind _fruit_party_2 (Variables|Default|GetFruit%20party))
  (bind _returnvalue (Utilities|Array|Length _fruit_party_2))
  (bind _returnvalue_2 (- _returnvalue 1))
  (bind _returnvalue_3 (Math|Random|RandomIntegerinRange 0 _returnvalue_2))
  (bind _output (Utilities|Array|Get(acopy) _fruit_party _returnvalue_3))
  (ChildActorComponent|SetChildActorClass (Variables|Default|GetTray1) _output)
  (ChildActorComponent|SetChildActorClass (Variables|Default|GetTray2) _output)
  (ChildActorComponent|SetChildActorClass (Variables|Default|GetTray3) _output)
  (ChildActorComponent|SetChildActorClass (Variables|Default|GetTray4) _output)
  (ChildActorComponent|SetChildActorClass (Variables|Default|GetTray5) _output)
  (ChildActorComponent|SetChildActorClass (Variables|Default|GetTray6) _output))