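; BP_HotPotato is a timed damage area, shown as a large explosion effect at its box's location.
; On BeginPlay it spawns the particle, waits for the Time duration (settable through SetTime), then destroys both the effect and itself.
; Box overlaps damage actors implementing IEnemy and play a hit sound, with the Enemies array ensuring each is hit only once.
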(event OnComponentBeginOverlap(Box)
  (params (OverlappedComponent :type Primitive%20Component%20Object%20Reference) (OtherActor :type Actor%20Object%20Reference) (OtherComp :type Primitive%20Component%20Object%20Reference) (OtherBodyIndex :type Integer) (bFromSweep :type Boolean) (SweepResult :type Hit%20Result%20Structure%20%28by%20ref%29))
  (CallFunction|DealDamage OtherActor (.impactpoint SweepResult)))

(event EventBeginPlay
  (bind _returnvalue (Effects|SpawnEmitteratLocation "/Game/Realistic_Starter_VFX_Pack_Vol2/Particles/Explosion/P_Explosion_Big_C.P_Explosion_Big_C" (Transformation|GetWorldLocation (Variables|Default|GetBox))))
  (Variables|Default|Setfire%20particle _returnvalue)
  (Utilities|FlowControl|Delay (Variables|Default|Gettime))
  (Components|DestroyComponent (Variables|Default|Getfire%20particle))
  (Actor|DestroyActor))

(event Collision|EventActorBeginOverlap
  (params (OtherActor :type Actor%20Object%20Reference)))

(event EventTick
  (params (DeltaSeconds :type Float%20%28single-precision%29)))

(fn ConstructionScript)

(fn SetTime
  (params (duration :type Float%20%28single-precision%29))
  (Variables|Default|Settime duration))

(fn HasEnemy
  (params (Actor :type Actor%20Object%20Reference))
  (return (Utilities|Set|Contains (Variables|Default|GetEnemies) Actor)))

(fn DealDamage
  (params (hit%20actor :type Actor%20Object%20Reference) (hit%20location :type Vector))
  (bind _hasenemy (CallFunction|HasEnemy hit%20actor))
  (if (and (not _hasenemy) (Utilities|DoesObjectImplementInterface hit%20actor "/Game/Characters/IEnemy.IEnemy_C"))
    (Utilities|Set|Add (Variables|Default|GetEnemies) hit%20actor)
    (Game|Damage|ApplyDamage hit%20actor (Variables|Default|GetDamage) 0 self)
    (Audio|SpawnSoundatLocation "/Game/Characters/Audio/BobOnHitSoundEffect.BobOnHitSoundEffect" hit%20location "0, 0, 0" 1.0 1.0 0.0 0 0)))