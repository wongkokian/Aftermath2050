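; BP_FireSword is a sword weapon whose Skill event fires a BP_Hadoken projectile from the sword, gated by a cooldown.
; The spawn point is offset from ItemMesh along the player 0 character mesh's forward vector, rotated 90 degrees about Z.
; That same direction becomes the projectile's FrontVector.
; A successful spawn clears CanShoot until a five-second timer calls Reset.
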(event EventBeginPlay)

(event Collision|EventActorBeginOverlap
  (params (OtherActor :type Actor%20Object%20Reference)))

(event EventTick
  (params (DeltaSeconds :type Float%20%28single-precision%29)))

(event EventSkill
  (bind _returnvalue (Game|GetPlayerCharacter 0))
  (bind _mesh (Variables|/Script/Engine.Character|GetMesh _returnvalue))
  (bind _returnvalue_2 (Math|Vector|GetForwardVector _mesh))
  (bind _returnvalue_3 (Math|Vector|RotateVectorAroundAxis _returnvalue_2 9e+01 "0, 0,1.000000"))
  (if (Variables|Default|GetcanShoot)
    (bind _returnvalue_4 (Game|SpawnActorfromClass "/Game/Weapon/BP_Hadoken.BP_Hadoken_C" (Math|Conversions|ToTransform(Vector) (+ (Transformation|GetWorldLocation (Variables|Default|GetItem%20Mesh)) (* _returnvalue_3 5e+01))) "Undefined" 0 0))
    (if (Utilities|IsValid _returnvalue_4)
      (Variables|/Game/Weapon/BP_Hadoken.BP_Hadoken_C|Setfront%20vector _returnvalue_4 _returnvalue_3)
      (Variables|Default|SetcanShoot false)
      (Utilities|Time|SetTimerbyFunctionName 0 "reset" 5.0))))

(fn ConstructionScript)

(fn Reset
  (Variables|Default|SetcanShoot true))