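; BP_Bubble is a bubble weapon actor that spawns a bubble particle effect and damages what overlaps it.
; After Duration, a timeline moves the effect along Z, then destroys it and the actor.
; An Enemy map stores last-hit times, so DealDamage repeats per target only after Interval, playing a hit sound each time.
; Begin overlap filters for IEnemy, while the per-tick Box overlap check applies only the interval test.
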(event EventBeginPlay
  (bind _returnvalue (Effects|SpawnEmitteratLocation "/Game/Realistic_Starter_VFX_Pack_Vol2/Particles/Water/P_Bubbles_A.P_Bubbles_A" (+ (Transformation|GetWorldLocation (Variables|Default|GetDefaultSceneRoot)) "0, 0,50.000000") "0, 0, 0" "10.000000,10.000000,10.000000"))
  (Variables|Default|Setbubble _returnvalue)
  (Utilities|FlowControl|Delay (Variables|Default|Getduration))
  (bind _move_down (Timeline|move%20down Play)
    (:Update
      (Transformation|AddRelativeLocation (Variables|Default|Getbubble) (Math|Vector|MakeVector 0.0 0.0 (* _move_down 1e+01)) false false))
    (:Finished
      (Components|DestroyComponent (Variables|Default|Getbubble))
      (Actor|DestroyActor))))

(event Collision|EventActorBeginOverlap
  (params (OtherActor :type Actor%20Object%20Reference))
  (if (Utilities|DoesObjectImplementInterface OtherActor "/Game/Characters/IEnemy.IEnemy_C")
    (if (not (Utilities|Map|Contains (Variables|Default|Getenemy) OtherActor))
      (CallFunction|DealDamage OtherActor)
      (else
        (bind _todamage (CallFunction|ToDealDamage OtherActor))
        (if _todamage
          (CallFunction|DealDamage OtherActor))))))

(event EventTick
  (params (DeltaSeconds :type Float%20%28single-precision%29))
  (for _array_element (Collision|GetOverlappingActors (Variables|Default|GetBox) 0 :!class /Script/Engine.PrimitiveComponent)
    (bind _todamage (CallFunction|ToDealDamage _array_element))
    (if _todamage
      (CallFunction|DealDamage _array_element))))

(fn ConstructionScript)

(fn ToDealDamage
  (params (enemy :type Actor%20Object%20Reference))
  (return (< (Variables|Default|GetInterval) (.seconds (- (Math|DateTime|Now) (.Value (Utilities|Map|Find (Variables|Default|Getenemy) enemy)))))))

(fn DealDamage
  (params (enemy :type Actor%20Object%20Reference))
  (Audio|PlaySoundatLocation "/Game/Characters/Audio/BobOnHitSoundEffect.BobOnHitSoundEffect" (Transformation|GetActorLocation enemy) "0, 0, 0" 1.0 1.0 0.0 0 0 enemy)
  (Game|Damage|ApplyDamage enemy (Variables|Default|GetDamage) 0 self)
  (Utilities|Map|Add (Variables|Default|Getenemy) enemy (Math|DateTime|Now)))