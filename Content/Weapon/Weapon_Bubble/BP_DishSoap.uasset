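; BP_DishSoap is an Uncommon weapon item that, once shot, turns into a bubble.
; It extends a parent item class, setting its scale, mass, launch angle, strength and rarity.
; Shooting calls the parent's projectile logic and starts a short timer to Destroy.
; Destroy plays a sound, traces down from the mesh, spawns BP_Bubble just above the hit point and removes the actor.
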(event EventBeginPlay
  (CallFunction|SetMass 1e+02)
  (Variables|Default|Setangle -2e+01)
  (Variables|Default|Setstrength 1e+03)
  (Variables|Default|SetRarirty "Uncommon")
  (|CallParentFunction))

(event Collision|EventActorBeginOverlap
  (params (OtherActor :type Actor%20Object%20Reference)))

(event EventTick
  (params (DeltaSeconds :type Float%20%28single-precision%29)))

(fn ConstructionScript
  (Transformation|SetActorScale3D "0.100000,0.100000,0.100000"))

(fn Destroy
  (bind _item_mesh (Variables|Default|GetItem%20Mesh))
  (bind _returnvalue (Transformation|GetWorldLocation _item_mesh))
  (Audio|PlaySoundatLocation "/Engine/EditorSounds/GamePreview/EjectFromPlayer.EjectFromPlayer" _returnvalue "0, 0, 0" 1.0 1.0 0.0 0 0 0)
  (bind _outhit (Collision|LineTraceByChannel _returnvalue (+ _returnvalue "0, 0,-1000.000000") "TraceTypeQuery1" false 0 "None"))
  (Game|SpawnActorfromClass "/Game/Weapon/Weapon_Bubble/BP_Bubble.BP_Bubble_C" (Math|Conversions|ToTransform(Vector) (+ (.location _outhit) "0, 0,50.000000")) "Undefined" 0 0)
  (Actor|DestroyActor))

(fn ShootProjectile
  (params (direction :type Vector :default "0, 0, 0") (location :type Vector :default "0, 0, 0"))
  (|CallParentFunction direction location)
  (Utilities|Time|SetTimerbyFunctionName 0 "destroy" 0.5))