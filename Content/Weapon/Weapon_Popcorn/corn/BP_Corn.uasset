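; BP_Corn is a rare corn projectile for the popcorn weapon, extending a parent projectile with its own mass, launch angle and strength.
; It overrides aim and launch to use the player controller's and pawn's forward vectors, ignoring the supplied direction when shooting.
; A one-second timer after firing triggers Explode, which plays effects, spawns a Kernel_spawner to scatter kernels and destroys the corn.
; A random point-on-sphere helper is defined but not called here.
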(event EventBeginPlay
  (CallFunction|SetMass 1e+02)
  (Variables|Default|Setangle -6e+01)
  (Variables|Default|Setstrength 1e+03)
  (Variables|Default|SetRarirty "Rare")
  (|CallParentFunction))

(event Collision|EventActorBeginOverlap
  (params (OtherActor :type Actor%20Object%20Reference))
  (|CallParentFunction OtherActor))

(event EventTick
  (params (DeltaSeconds :type Float%20%28single-precision%29)))

(event EventSetAim
  (params (location :type Vector :default "0, 0, 0") (direction :type Vector :default "0, 0, 0") (actors%20to%20ignore :type Array%20of%20Actor%20Object%20References))
  (|CallParentFunction location (Transformation|GetActorForwardVector (Game|GetPlayerController 0)) actors%20to%20ignore))

(fn ConstructionScript
  (Transformation|SetActorScale3D "3.000000,3.000000,3.000000"))

(fn ShootProjectile
  (params (direction :type Vector :default "0, 0, 0") (location :type Vector :default "0, 0, 0"))
  (|CallParentFunction (Transformation|GetActorForwardVector (Game|Player|GetPlayerPawn 0)) location)
  (Utilities|Time|SetTimerbyFunctionName self "Explode" 1.0))

(fn Explode
  (Variables|Default|Setcentre (Transformation|GetActorLocation))
  (Development|PrintString "Hello")
  (Audio|SpawnSoundatLocation "/Game/Characters/Audio/BobOnHitSoundEffect.BobOnHitSoundEffect" (Variables|Default|Getcentre) "0, 0, 0" 1.0 1.0 0.0 0 0)
  (Effects|SpawnEmitteratLocation "/Game/Realistic_Starter_VFX_Pack_Vol2/Particles/Explosion/P_Explosion_Big_A.P_Explosion_Big_A" (Variables|Default|Getcentre))
  (bind _returnvalue (Game|SpawnActorfromClass "/Game/Weapon/Weapon_Popcorn/kernel_spawner.kernel_spawner_C" (Math|Conversions|ToTransform(Vector) (Variables|Default|Getcentre)) "Undefined" 0 0))
  (Default|SpawnKernels _returnvalue (Variables|Default|Getcentre))
  (Actor|DestroyActor))

(fn GetPointinSphere
  (params (centre :type Vector))
  (LocalVariables|Setc centre)
  (LocalVariables|Settheta (Math|Random|RandomFloatinRange 0.0 3.6e+02))
  (LocalVariables|Setphi (Math|Random|RandomFloatinRange 0.0 1.8e+02))
  (LocalVariables|Setx (* (* (LocalVariables|Getradius) (Math|Trig|Sin(Degrees) (LocalVariables|Getphi))) (Math|Trig|Cos(Degrees) (LocalVariables|Gettheta))))
  (LocalVariables|Sety (* (* (LocalVariables|Getradius) (Math|Trig|Sin(Degrees) (LocalVariables|Getphi))) (Math|Trig|Sin(Degrees) (LocalVariables|Gettheta))))
  (LocalVariables|Setz (* (LocalVariables|Getradius) (Math|Trig|Cos(Degrees) (LocalVariables|Getphi))))
  (return (+ (Math|Vector|MakeVector (LocalVariables|Getx) (LocalVariables|Gety) (LocalVariables|Getz)) (LocalVariables|Getc))))