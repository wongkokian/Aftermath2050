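; Corn kernel actor for the popcorn weapon that lingers briefly, then moves out of view and destroys itself.
; On BeginPlay it sets a heavy mass, waits, disables collision, then runs the MoveDown timeline to offset its Z location each update until finished.
; Overlaps reach the parent class logic only for actors implementing IEnemy, and the player-collision check simply defers to the parent.
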(event EventBeginPlay
  (CallFunction|SetMass 4e+02)
  (Utilities|FlowControl|Delay 7.0)
  (CallFunction|SetCollisionDisabled)
  (bind _movedown (Timeline|move%20down Play)
    (:Update
      (Transformation|SetActorLocation (+ (Transformation|GetActorLocation) (Math|Vector|MakeVector 0.0 0.0 (* 5 _movedown))) false false))
    (:Finished
      (Actor|DestroyActor))))

(event Collision|EventActorBeginOverlap
  (params (OtherActor :type Actor%20Object%20Reference))
  (if (Utilities|DoesObjectImplementInterface OtherActor "/Game/Characters/IEnemy.IEnemy_C")
    (|CallParentFunction OtherActor)))

(event EventTick
  (params (DeltaSeconds :type Float%20%28single-precision%29)))

(fn ConstructionScript)

(fn IsCollidingPlayer
  (params (actor :type Actor%20Object%20Reference))
  (bind _isplayer (|CallParentFunction 0))
  (return _isplayer))