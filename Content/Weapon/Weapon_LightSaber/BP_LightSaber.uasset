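; BP_LightSaber is a Legendary lightsaber weapon with a Niagara laser blade and self-regenerating durability.
; Each tick, the blade's end point follows the Arrow's forward direction and its color is re-randomized.
; The Niagara component is made visible when an actor overlaps the saber.
; A looping timer restores durability up to a cap, spawning sparks on the item mesh with each gain.
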(event EventBeginPlay
  (Variables|Default|SetRarirty "Legendary")
  (|CallParentFunction)
  (Utilities|Time|SetTimerbyFunctionName 0 "regenerateDurability" 1e+01 true))

(event Collision|EventActorBeginOverlap
  (params (OtherActor :type Actor%20Object%20Reference))
  (Rendering|SetVisibility (Variables|Default|GetNiagara) true false)
  (|CallParentFunction OtherActor))

(event EventTick
  (params (DeltaSeconds :type Float%20%28single-precision%29))
  (bind _returnvalue (Math|Random|RandomFloatinRange 0.0 1.0))
  (bind _niagara (Variables|Default|GetNiagara))
  (Effects|Components|ParticleSystem|SetVectorParameter _niagara "laserEnd" (+ (* (Math|Vector|Normalize (Math|Vector|GetForwardVector (Variables|Default|GetArrow))) 1e+02) (Transformation|GetWorldLocation (Variables|Default|GetNiagara))))
  (Effects|Components|ParticleSystem|SetVectorParameter _niagara "Color" (Math|Vector|MakeVector _returnvalue _returnvalue _returnvalue)))

(fn ConstructionScript
  (Transformation|SetActorScale3D "0.080000,0.080000,0.300000"))

(fn RegenerateDurability
  (if (> (+ (Variables|Default|GetDurability) 1) 20)
    (Variables|Default|SetDurability 20)
    (else
      (Variables|Default|SetDurability (+ (Variables|Default|GetDurability) 1))
      (Effects|SpawnEmitterAttached "/Game/Realistic_Starter_VFX_Pack_Vol2/Particles/Sparks/P_Sparks_G.P_Sparks_G" (Variables|Default|GetItem%20Mesh) "None" (Transformation|GetWorldLocation (Variables|Default|GetItem%20Mesh)) "0, 0, 0" "2.000000,2.000000,2.000000"))))