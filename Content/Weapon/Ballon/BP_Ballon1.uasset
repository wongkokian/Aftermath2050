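; BP_Ballon1 is a proximity-triggered balloon actor that explodes when a Player-tagged actor overlaps its box.
; It starts with a random yaw, and the overlap sets a Triggered flag and plays a timeline that drives the actor's uniform scale.
; When the timeline finishes, Explode spawns an enlarged BP_HotBallon at the mesh location, assigns its damage and destroys this actor.
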(event OnComponentBeginOverlap(Box)
  (params (OverlappedComponent :type Primitive%20Component%20Object%20Reference) (OtherActor :type Actor%20Object%20Reference) (OtherComp :type Primitive%20Component%20Object%20Reference) (OtherBodyIndex :type Integer) (bFromSweep :type Boolean) (SweepResult :type Hit%20Result%20Structure%20%28by%20ref%29))
  (if (and (Actor|ActorHasTag OtherActor "Player") (not false))
    (Variables|Default|Settriggered true)
    (bind _newtrack_0 (Timeline|Timeline_0 Play)
      (:Update
        (Transformation|SetActorRelativeScale3D (Math|Vector|MakeVector _newtrack_0 _newtrack_0 _newtrack_0)))
      (:Finished
        (CallFunction|Explode)))))

(event EventBeginPlay
  (Transformation|SetRelativeRotation (Variables|Default|GetDefaultSceneRoot) (Math|Rotator|MakeRotator 0.0 0.0 (Math|Random|RandomFloatinRange -1.8e+02 1.8e+02)) false false))

(event Collision|EventActorBeginOverlap
  (params (OtherActor :type Actor%20Object%20Reference)))

(event EventTick
  (params (DeltaSeconds :type Float%20%28single-precision%29)))

(fn ConstructionScript)

(fn Explode
  (bind _returnvalue (Game|SpawnActorfromClass "/Game/Weapon/Weapon_Fruits/Vegetable/Potato/BP_HotBallon.BP_HotBallon_C" (Math|Transform|MakeTransform (Transformation|GetWorldLocation (Variables|Default|GetStaticMesh)) "0, 0, 0" "3.000000,3.000000,3.000000") "Undefined" 0 0))
  (Variables|/Game/Weapon/Weapon_Fruits/Vegetable/Potato/BP_HotBallon.BP_HotBallon_C|SetDamage _returnvalue 35.0)
  (Actor|DestroyActor))