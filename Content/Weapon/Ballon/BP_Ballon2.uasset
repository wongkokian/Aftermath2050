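; BP_Ballon2 is a player-triggered balloon weapon actor that flies off erratically, then bursts.
; It faces a random yaw on BeginPlay and starts a timeline when a Player-tagged actor overlaps its box.
; Timeline updates randomly jitter the root's yaw and push it along the arrow's forward vector without sweeping.
; When the timeline finishes, it spawns an enlarged BP_HotBallon at the mesh location, sets its damage and destroys itself.
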(event OnComponentBeginOverlap(Box)
  (params (OverlappedComponent :type Primitive%20Component%20Object%20Reference) (OtherActor :type Actor%20Object%20Reference) (OtherComp :type Primitive%20Component%20Object%20Reference) (OtherBodyIndex :type Integer) (bFromSweep :type Boolean) (SweepResult :type Hit%20Result%20Structure%20%28by%20ref%29))
  (bind _defaultsceneroot (Variables|Default|GetDefaultSceneRoot))
  (if (and (Actor|ActorHasTag OtherActor "Player") (not false))
    (Variables|Default|Settriggered true)
    (Timeline|Timeline_0 Play
      (:Update
        (Transformation|AddRelativeRotation _defaultsceneroot (Math|Rotator|MakeRotator 0.0 0.0 (* (Math|Random|RandomFloatinRange -1.0 1.0) 2e+01)) false false)
        (Transformation|AddWorldOffset _defaultsceneroot (* (Math|Vector|GetForwardVector (Variables|Default|GetArrow)) 5.0) false false))
      (:Finished
        (CallFunction|Explode)))))

(event EventBeginPlay
  (Transformation|SetRelativeRotation (Variables|Default|GetDefaultSceneRoot) (Math|Rotator|MakeRotator 0.0 0.0 (Math|Random|RandomFloatinRange -1.8e+02 1.8e+02)) false false))

(event Collision|EventActorBeginOverlap
  (params (OtherActor :type Actor%20Object%20Reference)))

(event EventTick
  (params (DeltaSeconds :type Float%20%28single-precision%29)))

(fn ConstructionScript)

(fn Explode
  (bind _returnvalue (Game|SpawnActorfromClass "/Game/Weapon/Weapon_Fruits/Vegetable/Potato/BP_HotBallon.BP_HotBallon_C" (Math|Transform|MakeTransform (Transformation|GetWorldLocation (Variables|Default|GetStaticMesh)) "0, 0, 0" "2.000000,2.000000,2.000000") "Undefined" 0 0))
  (Variables|/Game/Weapon/Weapon_Fruits/Vegetable/Potato/BP_HotBallon.BP_HotBallon_C|SetDamage _returnvalue 1e+01)
  (Actor|DestroyActor))