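; BP_Molotov is a Mythical-rarity molotov weapon that is launched and bursts into fire.
; BeginPlay sets its mass, angle, strength and rarity before running the parent weapon logic.
; ShootProjectile defers to the parent for the launch, then starts a one-second timer for Explode, so detonation is timed rather than impact-driven.
; Explode plays breaking glass and explosion effects, spawns BP_FireSpawner at its location, then destroys the actor.
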(event EventBeginPlay
  (CallFunction|SetMass 1e+02)
  (Variables|Default|Setangle -6e+01)
  (Variables|Default|Setstrength 1e+03)
  (Variables|Default|SetRarirty "Mythical")
  (|CallParentFunction))

(event Collision|EventActorBeginOverlap
  (params (OtherActor :type Actor%20Object%20Reference))
  (|CallParentFunction OtherActor))

(event EventTick
  (params (DeltaSeconds :type Float%20%28single-precision%29)))

(fn ConstructionScript)

(fn ShootProjectile
  (params (direction :type Vector :default "0, 0, 0"))
  (|CallParentFunction direction)
  (Utilities|Time|SetTimerbyFunctionName self "Explode" 1.0))

(fn Explode
  (bind _returnvalue (Transformation|GetActorLocation))
  (Audio|SpawnSoundatLocation "/Game/Characters/Audio/Breaking_glass_sound_effect.Breaking_glass_sound_effect" _returnvalue "0, 0, 0" 1.0 1.0 0.0 0 0)
  (Effects|SpawnEmitteratLocation "/Game/Realistic_Starter_VFX_Pack_Vol2/Particles/Explosion/P_Explosion_Big_A.P_Explosion_Big_A" _returnvalue)
  (Game|SpawnActorfromClass "/Game/BP_FireSpawner.BP_FireSpawner_C" (Math|Conversions|ToTransform(Vector) _returnvalue) "Undefined" 0 0)
  (Actor|DestroyActor))