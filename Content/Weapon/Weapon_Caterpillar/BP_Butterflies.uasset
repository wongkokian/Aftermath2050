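; BP_Butterflies is a Caterpillar weapon actor that creates a temporary butterfly zone which slows anything inside it.
; On BeginPlay it spawns a scaled butterfly particle emitter at its Box location, then removes the emitter and itself after Duration.
; Overlapping actors get their CustomTimeDilation sharply reduced, and leaving the Box restores it to normal.
; The destroy path contains no explicit reset of time dilation.
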(event OnComponentEndOverlap(Box)
  (params (OverlappedComponent :type Primitive%20Component%20Object%20Reference) (OtherActor :type Actor%20Object%20Reference) (OtherComp :type Primitive%20Component%20Object%20Reference) (OtherBodyIndex :type Integer))
  (Variables|/Script/Engine.Actor|SetCustomTimeDilation OtherActor 1.0))

(event EventBeginPlay
  (bind _returnvalue (Effects|SpawnEmitteratLocation "/Game/Realistic_Starter_VFX_Pack_Vol2/Particles/Environment/P_Butterfly.P_Butterfly" (Transformation|GetWorldLocation (Variables|Default|GetBox)) "0, 0, 0" "3.000000,3.000000,3.000000"))
  (Variables|Default|Setbutterfly _returnvalue)
  (Utilities|FlowControl|Delay (Variables|Default|Getduration))
  (Components|DestroyComponent (Variables|Default|Getbutterfly))
  (Actor|DestroyActor))

(event Collision|EventActorBeginOverlap
  (params (OtherActor :type Actor%20Object%20Reference))
  (Variables|/Script/Engine.Actor|SetCustomTimeDilation OtherActor 0.1))

(event EventTick
  (params (DeltaSeconds :type Float%20%28single-precision%29)))

(fn ConstructionScript)