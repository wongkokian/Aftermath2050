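; BP_Rack is a rack actor in the weapon folder that randomizes which of its child actor slots are populated.
; The construction script destroys most child actor components on a coin flip each, while ChildActor3 survives only rarely.
; The rolls use no seeded stream, so contents can change whenever construction reruns, and the event graph holds no active logic.
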(event EventBeginPlay)

(event Collision|EventActorBeginOverlap
  (params (OtherActor :type Actor%20Object%20Reference)))

(event EventTick
  (params (DeltaSeconds :type Float%20%28single-precision%29)))

(fn ConstructionScript
  (if (< (Math|Random|RandomFloatinRange 0.0 1.0) 0.9)
    (Components|DestroyComponent (Variables|Default|GetChildActor3)))
  (for _array_element (Utilities|Array|MakeArray (Variables|Default|GetChildActor1) (Variables|Default|GetChildActor) (Variables|Default|GetChildActor4) (Variables|Default|GetChildActor2) (Variables|Default|GetChildActor5) (Variables|Default|GetChildActor6) (Variables|Default|GetChildActor7) (Variables|Default|GetChildActor8) (Variables|Default|GetChildActor9) (Variables|Default|GetChildActor11) (Variables|Default|GetChildActor12) (Variables|Default|GetChildActor13) (Variables|Default|GetChildActor14) (Variables|Default|GetChildActor15) (Variables|Default|GetChildActor16))
    (if (Math|Random|RandomBool)
      (Components|DestroyComponent _array_element))))