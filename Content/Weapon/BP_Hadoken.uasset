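; BP_Hadoken is a fireball projectile that damages enemies and destroys itself after 2.5 seconds.
; Looping timers move it along FrontVector without sweep and billboard its Plane toward the player camera.
; When its Sphere overlaps an untagged-as-Player actor implementing IEnemy, it spawns an explosion, applies damage and destroys itself.
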(event OnComponentBeginOverlap(Sphere)
  (params (OverlappedComponent :type Primitive%20Component%20Object%20Reference) (OtherActor :type Actor%20Object%20Reference) (OtherComp :type Primitive%20Component%20Object%20Reference) (OtherBodyIndex :type Integer) (bFromSweep :type Boolean) (SweepResult :type Hit%20Result%20Structure%20%28by%20ref%29))
  (if (not (Actor|ActorHasTag OtherActor "Player"))
    (if (Utilities|DoesObjectImplementInterface OtherActor "/Game/Characters/IEnemy.IEnemy_C")
      (Effects|SpawnEmitteratLocation "/Game/Realistic_Starter_VFX_Pack_Vol2/Particles/Explosion/P_Explosion_Big_A.P_Explosion_Big_A" (Transformation|GetActorLocation) "0, 0, 0" "0.500000,0.500000,0.500000")
      (Game|Damage|ApplyDamage OtherActor 5e+01 0 0)
      (Actor|DestroyActor))))

(event EventBeginPlay
  (Utilities|Time|SetTimerbyFunctionName 0 "face fire ball" 0.01 true)
  (Utilities|Time|SetTimerbyFunctionName 0 "move fire ball" 0.01 true)
  (Utilities|FlowControl|Delay 2.5)
  (Actor|DestroyActor))

(event EventTick
  (params (DeltaSeconds :type Float%20%28single-precision%29)))

(fn ConstructionScript)

(fn FaceFireBall
  (bind _returnvalue (Game|GetPlayerCameraManager 0))
  (bind _returnvalue_2 (Transformation|GetActorLocation))
  (bind _returnvalue_3 (Camera|GetCameraLocation _returnvalue))
  (bind _returnvalue_4 (- _returnvalue_3 _returnvalue_2))
  (bind _returnvalue_5 (Math|Vector|Normalize _returnvalue_4))
  (bind _returnvalue_6 (Math|Conversions|RotationFromXVector _returnvalue_5))
  (Transformation|SetWorldRotation (Variables|Default|GetPlane) (Math|Rotator|MakeRotator (.roll _returnvalue_6) (+ (.pitch _returnvalue_6) 9e+01) (.yaw _returnvalue_6)) false false))

(fn MoveFireBall
  (Transformation|AddActorWorldOffset (* (Variables|Default|Getfront%20vector) 5.5)))