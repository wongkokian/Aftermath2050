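; BP_Trolley is a trolley actor that carries items attached to its Body sockets and lets one stored item be selected.
; PutItem and TakeItem move socket names between empty and taken lists, with a map linking sockets to items.
; Selection cycles with a negative-safe modulo, highlighting items through select/deselect messages, also triggered by actor overlap.
; IsEmpty actually reports whether any free slot remains.
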(event EventBeginPlay
  (for _array_element (Transformation|GetAllSocketNames (Variables|Default|GetBody))
    (Utilities|Array|Add (Variables|Default|GetemptySlots) _array_element)))

(event Collision|EventActorBeginOverlap
  (params (OtherActor :type Actor%20Object%20Reference))
  (if (> (Utilities|Array|Length (Variables|Default|GettakenSlots)) 0)
    (Variables|Default|Setselected 0)
    (CallFunction|HighlightCurrent)))

(event EventTick
  (params (DeltaSeconds :type Float%20%28single-precision%29)))

(event Collision|EventActorEndOverlap
  (params (OtherActor :type Actor%20Object%20Reference))
  (if (> (Utilities|Array|Length (Variables|Default|GettakenSlots)) 0)
    (CallFunction|UnhighlightCurrent)))

(fn ConstructionScript)

(fn TakeItem
  (bind _takenslots (Variables|Default|GettakenSlots))
  (bind _items (Variables|Default|Getitems))
  (if (!= (Utilities|Array|Length (Variables|Default|GettakenSlots)) 0)
    (LocalVariables|SetsocketName (Utilities|Array|Get(acopy) _takenslots (Variables|Default|Getselected)))
    (bind _output_get (LocalVariables|SetitemSelected (.Value (Utilities|Map|Find _items (LocalVariables|GetsocketName)))))
    (Transformation|DetachFromActor _output_get "KeepWorld" "KeepWorld" "KeepWorld")
    (Utilities|Map|Remove _items (LocalVariables|GetsocketName))
    (Utilities|Array|RemoveItem _takenslots (LocalVariables|GetsocketName))
    (Utilities|Array|Add (Variables|Default|GetemptySlots) (LocalVariables|GetsocketName))
    (Class|BPIInteractable|DeselectinTrolley(Message) _output_get)
    (return _output_get true)
    (else
      (return 0 false))))

(fn IsEmpty
  (return (> (Utilities|Array|Length (Variables|Default|GetemptySlots)) 0)))

(fn PutItem
  (params (item :type Actor%20Object%20Reference))
  (bind _emptyslots (Variables|Default|GetemptySlots))
  (bind _output (Utilities|Array|Get(acopy) _emptyslots))
  (Transformation|AttachComponentToComponent item (Variables|Default|GetBody) _output "SnapToTarget" "SnapToTarget" "KeepWorld" true)
  (Utilities|Map|Add (Variables|Default|Getitems) _output item)
  (Utilities|Array|Add (Variables|Default|GettakenSlots) _output)
  (Utilities|Array|RemoveItem (Variables|Default|GetemptySlots) _output)
  (CallFunction|HighlightCurrent))

(fn HighlightCurrent
  (Class|BPIInteractable|SelectinTrolley(Message) (.Value (Utilities|Map|Find (Variables|Default|Getitems) (Utilities|Array|Get(acopy) (Variables|Default|GettakenSlots) (Variables|Default|Getselected))))))

(fn UnhighlightCurrent
  (Class|BPIInteractable|DeselectinTrolley(Message) (.Value (Utilities|Map|Find (Variables|Default|Getitems) (Utilities|Array|Get(acopy) (Variables|Default|GettakenSlots) (Variables|Default|Getselected))))))

(fn IncreaseSelected
  (bind _takenslots (Variables|Default|GettakenSlots))
  (bind _returnvalue (Utilities|Array|Length _takenslots))
  (if (> _returnvalue 0)
    (CallFunction|UnhighlightCurrent)
    (bind _res (CallFunction|Modulo (+ (Variables|Default|Getselected) 1) _returnvalue))
    (Variables|Default|Setselected _res)
    (CallFunction|HighlightCurrent)))

(fn DecreaseSelected
  (bind _takenslots (Variables|Default|GettakenSlots))
  (bind _returnvalue (Utilities|Array|Length _takenslots))
  (if (> _returnvalue 0)
    (CallFunction|UnhighlightCurrent)
    (bind _res (CallFunction|Modulo (+ (Variables|Default|Getselected) -1) _returnvalue))
    (Variables|Default|Setselected _res)
    (CallFunction|HighlightCurrent)))

(fn Modulo
  (params (x :type Integer) (n :type Integer))
  (return (Math|Integer|%(Integer) (+ (Math|Integer|%(Integer) x n) n) n)))