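; Dungeon generator actor that arranges five pre-built rooms (donut shop, SP, dining, restaurant, warehouse) into a randomized linked chain at BeginPlay.
; It shuffles room structs, measures bounds, picks orientations that define left and right walls, then spaces rooms along X with random Y offsets.
; Doors replace facing wall pieces, and spawned floor-tile meshes form corridors between rooms.
; Door_Activate swings a door's child SceneComponent open through a timeline.
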(event Custom|Door_Activate
  (params (Doorwall :type Primitive%20Component%20Object%20Reference))
  ;[1 1 1] Activate open and closing of door
  (Development|PrintString "cast succeeded")
  (bind _doorhinge (CallFunction|OpenandCloseDoor Doorwall))
  (if (Utilities|IsValid _doorhinge)
    (bind _opendoor (Timeline|Open%20and%20Close%20Door PlayFromStart)
      (:Update
        (Transformation|SetRelativeRotation _doorhinge (Math|Rotator|MakeRotator 0.0 0.0 _opendoor) false false)))))

(event EventBeginPlay
  ;[1 1 1] Set DonutRoom Walls
  (Variables|Default|SetDonutRoomStruct (Utilities|Struct|MakeRoom_Struct 0 (Utilities|Array|MakeArray 0 2) 0 0 -1.0 -1.0 (Utilities|Array|MakeArray (Variables|Components|Get0_Wall1) (Variables|Components|Get0_Wall6) (Variables|Components|Get0_Wall5)) (Utilities|Array|MakeArray (Variables|Components|Get1_Wall7) (Variables|Components|Get1_Wall8)) (Utilities|Array|MakeArray (Variables|Components|Get2_Wall1) (Variables|Components|Get2_Wall2) (Variables|Components|Get2_Wall3)) (Utilities|Array|MakeArray (Variables|Components|Get3_Wall9) (Variables|Components|Get3_Wall10)) (Variables|Default|GetDonutShop_Base) (Variables|Components|GetDonut_Door) (Variables|Default|GetDonut_Door1) "0.000000,0.000000,0.000000"))
  ;[1 1 1] Ser SPRoom Walls
  (Variables|Default|SetSPRoomStruct (Utilities|Struct|MakeRoom_Struct 0 (Utilities|Array|MakeArray 0 2) 0 0 -1.0 -1.0 (Utilities|Array|MakeArray (Variables|Components|GetSP0_Wall1) (Variables|Components|GetSP0_Wall3) (Variables|Components|GetSP0_Wall2)) (Utilities|Array|MakeArray (Variables|Components|GetSP1_Wall1) (Variables|Components|GetSP1_Wall3) (Variables|Components|GetSP1_Wall2)) (Utilities|Array|MakeArray (Variables|Components|GetSP2_Wall1) (Variables|Components|GetSP2_Wall3) (Variables|Components|GetSP2_Wall2)) (Utilities|Array|MakeArray (Variables|Components|GetSP3_Wall11) (Variables|Components|GetSP3_Wall13) (Variables|Components|GetSP3_Wall12)) (Variables|Components|GetSP_Base) (Variables|Default|GetSP_Door) (Variables|Default|GetSP_Door1) "0.000000,0.000000,0.000000"))
  ;[1 1 1] Ser SPRoom Walls
  (Variables|Default|SetDiningRoomStruct (Utilities|Struct|MakeRoom_Struct 0 (Utilities|Array|MakeArray 1 3) 0 0 0.0 0.0 (Utilities|Array|MakeArray (Variables|Default|GetD0_Wall4) (Variables|Default|GetD0_Wall7) (Variables|Default|GetD0_Wall8) (Variables|Default|GetD0_Wall5) (Variables|Default|GetD0_Wall6)) (Utilities|Array|MakeArray (Variables|Default|GetD1_Wall14) (Variables|Default|GetD1_Wall17) (Variables|Default|GetD1_Wall18) (Variables|Default|GetD1_Wall15) (Variables|Default|GetD1_Wall16)) (Utilities|Array|MakeArray 0 (Variables|Default|GetD2_Wall13) (Variables|Default|GetD2_Wall11) (Variables|Default|GetD2_Wall9) (Variables|Default|GetD2_Wall12)) (Utilities|Array|MakeArray (Variables|Default|GetD3_Wall14) (Variables|Default|GetD3_Wall17) (Variables|Default|GetD3_Wall18) (Variables|Default|GetD3_Wall16) (Variables|Default|GetD3_Wall15)) (Variables|Default|GetDining_Base) (Variables|Default|GetD_Door) (Variables|Default|GetD_Door1) "0.000000,0.000000,0.000000"))
  ;[1 1 1] Ser SPRoom Walls
  (Variables|Default|SetRestaurantRoomStruct (Utilities|Struct|MakeRoom_Struct 0 (Utilities|Array|MakeArray 0 2) 0 0 0.0 0.0 (Utilities|Array|MakeArray (Variables|Default|GetR0_Wall4) (Variables|Default|GetR0_Wall6) (Variables|Default|GetR0_Wall5)) (Utilities|Array|MakeArray (Variables|Default|GetR1_Wall4) (Variables|Default|GetR1_Wall7) (Variables|Default|GetR1_Wall8)) (Utilities|Array|MakeArray (Variables|Default|GetR2_Wall5) (Variables|Default|GetR2_Wall6) (Variables|Default|GetR2_Wall4)) (Utilities|Array|MakeArray (Variables|Default|GetR3_Wall15) (Variables|Default|GetR3_Wall17) (Variables|Default|GetR3_Wall18)) (Variables|Default|GetResto_Base) (Variables|Default|GetR_Door) (Variables|Default|GetR_Door1) "0.000000,0.000000,0.000000"))
  ;[1 1 1] Set DonutRoom Walls
  (Variables|Default|SetWarehouseRoomStruct (Utilities|Struct|MakeRoom_Struct 0 (Utilities|Array|MakeArray 1 3) 0 0 0.0 0.0 (Utilities|Array|MakeArray (Variables|Default|GetW0_Wall2) (Variables|Default|GetW0_Wall7) (Variables|Default|GetW0_Wall8)) (Utilities|Array|MakeArray (Variables|Default|GetW1_Wall9) (Variables|Default|GetW1_Wall10)) (Utilities|Array|MakeArray (Variables|Default|GetW2_Wall4) (Variables|Default|GetW2_Wall6) (Variables|Default|GetW2_Wall5)) (Utilities|Array|MakeArray (Variables|Default|GetW3_Wall11) (Variables|Default|GetW3_Wall12)) (Variables|Default|GetWarehouse_Base) (Variables|Default|GetW_Door) (Variables|Default|GetW_Door1) "0.000000,0.000000,0.000000"))
  ;[1 1 1] Add all room structs into RoomStructs Array and shuffle the array
  (bind _output_get (Variables|Default|SetRoomStructs (Utilities|Array|MakeArray (Variables|Default|GetDonutRoomStruct) (Variables|Default|GetSPRoomStruct) (Variables|Default|GetDiningRoomStruct) (Variables|Default|GetRestaurantRoomStruct) (Variables|Default|GetWarehouseRoomStruct))))
  (Utilities|Array|Shuffle _output_get)
  ;[1 1 1] For each room: Set Orientation and Set Width and Length
  (for (_array_element _array_index) _output_get
    (bind _new_room_struct (CallFunction|SetLengthandWidth _array_element))
    (bind _structout (Utilities|Struct|SetmembersinRoom_Struct _array_element (.length _new_room_struct) (.width _new_room_struct)))
    (bind _new_room_struct_2 (CallFunction|SetOrientation _structout))
    (Utilities|Array|SetArrayElem (Variables|Default|GetRoomStructs) _array_index _new_room_struct_2))
  ;[1 1 1] Set location of each room iteratively
  (Variables|Default|SetPreviousRoomStruct (Utilities|Array|Get(acopy) (Variables|Default|GetRoomStructs)))
  (for (_array_element_2 _array_index_2) _output_get
    (bind _new_room_struct_3 (CallFunction|SetLocation _array_element_2 (Variables|Default|GetPreviousRoomStruct) _array_index_2))
    (Variables|Default|SetPreviousRoomStruct _new_room_struct_3)
    (Utilities|Array|SetArrayElem (Variables|Default|GetRoomStructs) _array_index_2 _new_room_struct_3))
  ;[1 1 1] Spawn doors
  (Variables|Default|SetPreviousRoomStruct (Utilities|Array|Get(acopy) (Variables|Default|GetRoomStructs)))
  (for (_array_element_3 _array_index_3) (Variables|Default|GetRoomStructs)
    (CallFunction|ReplaceDoors (Variables|Default|GetPreviousRoomStruct) _array_element_3 _array_index_3)
    (Variables|Default|SetPreviousRoomStruct _array_element_3))
  (Variables|Default|SetPreviousRoomStruct (Utilities|Array|Get(acopy) (Variables|Default|GetRoomStructs)))
  (for _array_element_4 (Variables|Default|GetRoomStructs)
    (CallFunction|CreateCorridor (Variables|Default|GetPreviousRoomStruct) _array_element_4 (Variables|Default|GetLeftTile) (Variables|Default|GetRightTile))
    (Variables|Default|SetPreviousRoomStruct _array_element_4)))

(event Collision|EventActorBeginOverlap
  (params (OtherActor :type Actor%20Object%20Reference)))

(event EventTick
  (params (DeltaSeconds :type Float%20%28single-precision%29)))

(fn ConstructionScript)

(fn SetOrientation
  (params (Room%20Struct :type Room%20Struct%20Structure))
  (bind (_orientation _doorwalls _leftwalls _rightwalls _length _width _0_walls _1_walls _2_walls _3_walls _basecomponent) (Utilities|Struct|BreakRoom_Struct Room%20Struct))
  (bind (_orientation_2 _doorwalls_2 _leftwalls_2 _rightwalls_2 _length_2 _width_2 _0_walls_2 _1_walls_2 _2_walls_2 _3_walls_2) (Utilities|Struct|BreakRoom_Struct Room%20Struct))
  ;[1 1 1] Randomly sets orientation of room
  (Utilities|Struct|SetmembersinRoom_Struct Room%20Struct (Utilities|Array|Get(acopy) _doorwalls (Math|Random|RandomInteger (Utilities|Array|Length _doorwalls))))
  (Transformation|SetWorldRotation _basecomponent (Math|Rotator|MakeRotator 0.0 0.0 (* (.orientation Room%20Struct) 9e+01)) false false)
  ;[1 1 1] Based on orientation - set Right and Left Wall values
  (switch int (.orientation Room%20Struct)
    (:Default
      _)
    (:0
      _)
    (:1
      (bind _structout (Utilities|Struct|SetmembersinRoom_Struct Room%20Struct _3_walls_2 _1_walls_2))
      (return _structout))
    (:2
      (bind _structout_2 (Utilities|Struct|SetmembersinRoom_Struct Room%20Struct _0_walls_2 _2_walls_2))
      (return _structout_2))
    (:3
      (bind _structout_3 (Utilities|Struct|SetmembersinRoom_Struct Room%20Struct _1_walls_2 _3_walls_2))
      (return _structout_3)))
  (bind _structout_4 (Utilities|Struct|SetmembersinRoom_Struct Room%20Struct _2_walls_2 _0_walls_2))
  (return _structout_4))

(fn SetLengthandWidth
  (params (Room%20Struct :type Room%20Struct%20Structure))
  (bind _basecomponent (Utilities|Struct|BreakRoom_Struct Room%20Struct))
  (bind _boxextent (Collision|GetComponentBounds _basecomponent))
  (bind _structout (Utilities|Struct|SetmembersinRoom_Struct Room%20Struct (.y _boxextent) (.x _boxextent)))
  (return _structout))

(fn SetLocation
  (params (Room%20Struct :type Room%20Struct%20Structure) (Previous%20Room%20Struct :type Room%20Struct%20Structure) (RoomOrder :type Integer))
  (bind (_orientation _doorwalls _leftwalls _rightwalls _length _width _0_walls _1_walls _2_walls _3_walls _basecomponent) (Utilities|Struct|BreakRoom_Struct Room%20Struct))
  (bind (_orientation_2 _doorwalls_2 _leftwalls_2 _rightwalls_2 _length_2 _width_2 _0_walls_2 _1_walls_2 _2_walls_2 _3_walls_2 _basecomponent_2 _leftdoor _rightdoor _location) (Utilities|Struct|BreakRoom_Struct Previous%20Room%20Struct))
  (bind _returnvalue (+ _length _length_2 -1e+03))
  ;[1 1 1] If the first room
  (if (== RoomOrder 0)
    (bind _structout (Utilities|Struct|SetmembersinRoom_Struct Room%20Struct (Math|Vector|MakeVector 0.0 0.0 (.yaw (Transformation|GetWorldRotation _basecomponent)))))
    (Transformation|SetWorldLocation _basecomponent (.location _structout) false false)
    (return Room%20Struct)
    (else
      ;[1 1 1] If not the first room (i.e., x value is not fixed and depends on previous room)
      (bind _structout_2 (Utilities|Struct|SetmembersinRoom_Struct Room%20Struct (Math|Vector|MakeVector (+ (/ _width 2.0) (.x _location) (/ _width_2 2.0) 2.75e+03) (+ (- (* _returnvalue (Math|Random|RandomFloat)) (/ _returnvalue 2.0)) (.y _location)) (.z (Transformation|GetWorldLocation _basecomponent_2)))))
      (Transformation|SetWorldLocation _basecomponent (Math|Vector|MakeVector (.x (.location _structout_2)) (.y (.location _structout_2)) 0.0) false false)
      (return Room%20Struct))))

(fn ReplaceDoors
  (params (Previous%20Room%20Struct :type Room%20Struct%20Structure) (Room%20Struct :type Room%20Struct%20Structure) (RoomOrder :type Integer))
  (bind (_orientation _doorwalls _leftwalls _rightwalls _length _width _0_walls _1_walls _2_walls _3_walls _basecomponent _leftdoor _rightdoor) (Utilities|Struct|BreakRoom_Struct Previous%20Room%20Struct))
  (bind (_orientation_2 _doorwalls_2 _leftwalls_2 _rightwalls_2 _length_2 _width_2 _0_walls_2 _1_walls_2 _2_walls_2 _3_walls_2 _basecomponent_2 _leftdoor_2) (Utilities|Struct|BreakRoom_Struct Room%20Struct))
  (if (== RoomOrder 0)
    ;[1 1 1] If it is the first room, destroy the left door
    (for _array_element (Components|GetChildrenComponents _leftdoor_2 true)
      (Components|DestroyComponent _array_element))
    (Components|DestroyComponent _leftdoor_2)
    (else
      ;[1 1 1] Set Previous Room Walls
      (bind _output_get (Variables|Components|SetWallToDestroy (Utilities|Array|Get(acopy) _rightwalls (Math|Random|RandomInteger 0))))
      (Transformation|SetWorldLocation _rightdoor (Transformation|GetWorldLocation _output_get) false false)
      (Transformation|SetWorldRotation _rightdoor "0.000000,180.000000, 0" false false)
      (Components|DestroyComponent _output_get)
      ;[1 1 1] replacing door for current room (LeftWalls)
      (bind _output_get_2 (Variables|Default|SetCurrWallToDestroy (Utilities|Array|Get(acopy) _leftwalls_2 (Math|Random|RandomInteger 0))))
      (Transformation|SetWorldLocation _leftdoor_2 (Transformation|GetWorldLocation _output_get_2) false false)
      (Transformation|SetWorldRotation _leftdoor_2 (Math|Rotator|MakeRotator 0.0 0.0 0.0) false false)
      (Components|DestroyComponent _output_get_2))))

(fn OpenandCloseDoor
  (params (DoorWall :type Primitive%20Component%20Object%20Reference))
  (bind _array_element (Utilities|Array|ForEachLoopwithBreak (Components|GetChildrenComponents DoorWall false))
    (:LoopBody
      (if (== (Utilities|GetClass _array_element) "/Script/Engine.SceneComponent")
        (Development|PrintString (Utilities|GetDisplayName _array_element))
        (return _array_element)))
    (:Completed
      (Development|PrintString "why're u trying to open a non-door")
      (return 0))))

(fn CreateCorridor
  (params (Previous%20Room%20Struct :type Room%20Struct%20Structure) (Room%20Struct :type Room%20Struct%20Structure) (Left%20Tile :type Float%20%28single-precision%29) (Right%20Tile :type Float%20%28single-precision%29))
  (bind (_orientation _doorwalls _leftwalls _rightwalls _length _width _0_walls _1_walls _2_walls _3_walls _basecomponent _leftdoor _rightdoor) (Utilities|Struct|BreakRoom_Struct Previous%20Room%20Struct))
  (bind (_orientation_2 _doorwalls_2 _leftwalls_2 _rightwalls_2 _length_2 _width_2 _0_walls_2 _1_walls_2 _2_walls_2 _3_walls_2 _basecomponent_2 _leftdoor_2) (Utilities|Struct|BreakRoom_Struct Room%20Struct))
  (bind _returnvalue (Transformation|GetWorldLocation _rightdoor))
  (bind _returnvalue_2 (Transformation|GetWorldLocation _leftdoor_2))
  (bind _returnvalue_3 (Transformation|GetWorldLocation _leftdoor_2))
  (bind _returnvalue_4 (+ (.x _returnvalue) 4e+02))
  (bind _returnvalue_5 (+ (.y _returnvalue) -5e+02))
  (bind _returnvalue_6 (+ (.y _returnvalue_2) 5e+02))
  (if (not (== _basecomponent _basecomponent_2))
    ;[1 1 1] Statrting platforms
    (bind _returnvalue_7 (AddComponent|AddStaticMeshComponent false))
    (Components|StaticMesh|SetStaticMesh _returnvalue_7 "/Game/AssetsvilleTown/Meshes/BuildingTilset/SM_floor_01.SM_floor_01")
    (Transformation|SetWorldScale3D _returnvalue_7 "2.000000,2.000000,1.000000")
    (Transformation|SetWorldLocation _returnvalue_7 (Math|Vector|MakeVector _returnvalue_4 _returnvalue_5 -0.1) false false)
    (Variables|Default|SetLeftTile _returnvalue_5)
    (bind _returnvalue_8 (AddComponent|AddStaticMeshComponent false))
    (Components|StaticMesh|SetStaticMesh _returnvalue_8 "/Game/AssetsvilleTown/Meshes/BuildingTilset/SM_floor_01.SM_floor_01")
    (Transformation|SetWorldScale3D _returnvalue_8 "2.000000,2.000000,1.000000")
    (Transformation|SetWorldLocation _returnvalue_8 (Math|Vector|MakeVector (+ (.x _returnvalue_2) -4e+02) _returnvalue_6 -0.1) false false)
    (bind _returnvalue_9 (AddComponent|AddStaticMeshComponent false))
    (Components|StaticMesh|SetStaticMesh _returnvalue_9 "/Game/AssetsvilleTown/Meshes/BuildingTilset/SM_floor_01.SM_floor_01")
    (Transformation|SetWorldScale3D _returnvalue_9 "2.000000,2.000000,1.000000")
    (Transformation|SetWorldLocation _returnvalue_9 (Math|Vector|MakeVector (+ (.x _returnvalue_3) -1.1e+03) (+ (.y _returnvalue_3) 5e+02) -0.1) false false)
    (bind _output_get (Variables|Default|SetRightTile _returnvalue_6))
    (if (> (Variables|Default|GetLeftTile) (Variables|Default|GetRightTile))
      (while (< (+ (Variables|Default|GetRightTile) 2e+02) (+ (Variables|Default|GetLeftTile) -2e+02))
        (bind _returnvalue_10 (AddComponent|AddStaticMeshComponent false))
        (Components|StaticMesh|SetStaticMesh _returnvalue_10 "/Game/AssetsvilleTown/Meshes/BuildingTilset/SM_floor_01.SM_floor_01")
        (Transformation|SetWorldScale3D _returnvalue_10 "2.000000,2.000000,1.000000")
        (Transformation|SetWorldLocation _returnvalue_10 (Math|Vector|MakeVector _returnvalue_4 (+ (Variables|Default|GetLeftTile) -4e+02) -0.1) false false)
        (Variables|Default|SetLeftTile (+ (Variables|Default|GetLeftTile) -4e+02)))
      (else
        (while (> (- (Variables|Default|GetRightTile) 2e+02) (+ (Variables|Default|GetLeftTile) 2e+02))
          (bind _returnvalue_11 (AddComponent|AddStaticMeshComponent false))
          (Components|StaticMesh|SetStaticMesh _returnvalue_11 "/Game/AssetsvilleTown/Meshes/BuildingTilset/SM_floor_01.SM_floor_01")
          (Transformation|SetWorldScale3D _returnvalue_11 "2.000000,2.000000,1.000000")
          (Transformation|SetWorldLocation _returnvalue_11 (Math|Vector|MakeVector _returnvalue_4 (+ (Variables|Default|GetLeftTile) 4e+02) -0.1) false false)
          (Variables|Default|SetLeftTile (+ (Variables|Default|GetLeftTile) 4e+02)))))))