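; Hinged door that an OpenDoor event swings open in a direction set by which side box the player stands in.
; Timelines rotate the hinge yaw, multiplied by a direction sign, playing forward to open and in reverse to close.
; It closes automatically when Bob leaves a box and the player is not in the other one.
; The open sound plays on every OpenDoor call, even when nothing moves.
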(event OnComponentEndOverlap(LeftBox)
  (params (OverlappedComponent :type Primitive%20Component%20Object%20Reference) (OtherActor :type Actor%20Object%20Reference) (OtherComp :type Primitive%20Component%20Object%20Reference) (OtherBodyIndex :type Integer))
  (if (== (Utilities|GetClass OtherActor) "/Game/Characters/Bob.Bob_C")
    (if (and (not (Variables|Default|GetClosed)) (not (Collision|IsOverlappingActor (Variables|Default|GetRightBox) (Game|GetPlayerCharacter 0) :!class /Script/Engine.PrimitiveComponent)))
      (Variables|Default|SetClosed true)
      (Audio|PlaySound2D "/Game/BGM/door_close_sound.door_close_sound" 1.0 1.0 -1.0 0 0)
      (bind _opendoor (Timeline|Timeline_2 ReverseFromEnd)
        (:Update
          (Transformation|SetRelativeRotation (Variables|Default|GetScene%28Hinge%29) (Math|Rotator|MakeRotator 0.0 0.0 (* _opendoor (Variables|Default|GetRotationDirection))) false false))))))

(event OnComponentEndOverlap(RightBox)
  (params (OverlappedComponent :type Primitive%20Component%20Object%20Reference) (OtherActor :type Actor%20Object%20Reference) (OtherComp :type Primitive%20Component%20Object%20Reference) (OtherBodyIndex :type Integer))
  (if (== (Utilities|GetClass OtherActor) "/Game/Characters/Bob.Bob_C")
    (if (and (not (Collision|IsOverlappingActor (Variables|Default|GetLeftBox) (Game|GetPlayerCharacter 0) :!class /Script/Engine.PrimitiveComponent)) (not (Variables|Default|GetClosed)))
      (Variables|Default|SetClosed true)
      (Audio|PlaySound2D "/Game/BGM/door_close_sound.door_close_sound" 1.0 1.0 -1.0 0 0)
      (bind _opendoor (Timeline|Timeline_3 ReverseFromEnd)
        (:Update
          (Transformation|SetRelativeRotation (Variables|Default|GetScene%28Hinge%29) (Math|Rotator|MakeRotator 0.0 0.0 (* _opendoor (Variables|Default|GetRotationDirection))) false false))))))

(event Custom|OpenDoor
  (Audio|PlaySound2D "/Game/BGM/open_door_sound.open_door_sound" 1.0 1.0 0.5 0 0)
  (if (Variables|Default|GetClosed)
    (if (Collision|IsOverlappingActor (Variables|Default|GetLeftBox) (Game|GetPlayerCharacter 0) :!class /Script/Engine.PrimitiveComponent)
      (Variables|Default|SetRotationDirection -1.0)
      (Variables|Default|SetClosed false)
      (Utilities|FlowControl|Sequence
        (:then_1
          (bind _opendoor (Timeline|Timeline_1 PlayFromStart)
            (:Update
              (Transformation|SetRelativeRotation (Variables|Default|GetScene%28Hinge%29) (Math|Rotator|MakeRotator 0.0 0.0 (* _opendoor (Variables|Default|GetRotationDirection))) false false)))))
      (elif (Collision|IsOverlappingActor (Variables|Default|GetRightBox) (Game|GetPlayerCharacter 0) :!class /Script/Engine.PrimitiveComponent)
        (Variables|Default|SetRotationDirection 1.0)
        (Variables|Default|SetClosed false)
        (Utilities|FlowControl|Sequence
          (:then_1
            (bind _opendoor_2 (Timeline|Timeline_0 PlayFromStart)
              (:Update
                (Transformation|SetRelativeRotation (Variables|Default|GetScene%28Hinge%29) (Math|Rotator|MakeRotator 0.0 0.0 (* _opendoor_2 (Variables|Default|GetRotationDirection))) false false)))))))))

(event EventBeginPlay)

(event Collision|EventActorBeginOverlap
  (params (OtherActor :type Actor%20Object%20Reference)))

(event EventTick
  (params (DeltaSeconds :type Float%20%28single-precision%29)))

(fn ConstructionScript)