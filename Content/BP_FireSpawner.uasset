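; BP_FireSpawner spreads fire outward from its placed location by spawning BP_Fire actors on a grid.
; A looping timer spawns fire at each pending cell, snapped to the surface hit by a vertical line trace.
; Each cell then queues unused orthogonal neighbours through random rolls, tracked in SpawnedLocation to avoid repeats.
; The spread probability drops slightly with every fire, so growth tapers off.
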(event EventBeginPlay
  (Variables|Default|Setorigin (Transformation|GetWorldLocation (Variables|Default|GetDefaultSceneRoot)))
  (Utilities|Array|Add :TargetArray (Variables|Default|GetlocationToSpawn))
  (Utilities|Time|SetTimerbyFunctionName 0 "spawnFire" 0.1 true)
  (if (== (Utilities|Array|Length (Variables|Default|GetlocationToSpawn)) 0)
    (Actor|DestroyActor)))

(event Collision|EventActorBeginOverlap
  (params (OtherActor :type Actor%20Object%20Reference)))

(event EventTick
  (params (DeltaSeconds :type Float%20%28single-precision%29)))

(fn ConstructionScript)

(fn GetPotentialSpawnPoint
  (params (current :type Vector))
  (bind _locationtospawn (Variables|Default|GetlocationToSpawn))
  (bind _spawnedlocation (Variables|Default|GetspawnedLocation))
  (LocalVariables|Settemp current)
  (for _index (range 0 3)
    (switch int _index
      (:0
        (bind _isvalid (CallFunction|IsValid (+ (LocalVariables|Gettemp) "1.000000, 0, 0")))
        (if _isvalid
          (bind _tospawn (CallFunction|ToSpawn))
          (if _tospawn
            (Utilities|Array|Add _locationtospawn (+ (LocalVariables|Gettemp) "1.000000, 0, 0"))
            (Utilities|Set|Add _spawnedlocation (+ (LocalVariables|Gettemp) "1.000000, 0, 0")))))
      (:1
        (bind _isvalid_2 (CallFunction|IsValid (+ (LocalVariables|Gettemp) "-1.000000, 0, 0")))
        (if _isvalid_2
          (bind _tospawn_2 (CallFunction|ToSpawn))
          (if _tospawn_2
            (Utilities|Array|Add _locationtospawn (+ (LocalVariables|Gettemp) "-1.000000, 0, 0"))
            (Utilities|Set|Add _spawnedlocation (+ (LocalVariables|Gettemp) "-1.000000, 0, 0")))))
      (:2
        (bind _isvalid_3 (CallFunction|IsValid (+ (LocalVariables|Gettemp) "0.000000,-1.000000, 0")))
        (if _isvalid_3
          (bind _tospawn_3 (CallFunction|ToSpawn))
          (if _tospawn_3
            (Utilities|Array|Add _locationtospawn (+ (LocalVariables|Gettemp) "0.000000,-1.000000, 0"))
            (Utilities|Set|Add _spawnedlocation (+ (LocalVariables|Gettemp) "0.000000,-1.000000, 0")))))
      (:3
        (bind _isvalid_4 (CallFunction|IsValid (+ (LocalVariables|Gettemp) "0.000000,1.000000, 0")))
        (if _isvalid_4
          (bind _tospawn_4 (CallFunction|ToSpawn))
          (if _tospawn_4
            (Utilities|Array|Add _locationtospawn (+ (LocalVariables|Gettemp) "0.000000,1.000000, 0"))
            (Utilities|Set|Add _spawnedlocation (+ (LocalVariables|Gettemp) "0.000000,1.000000, 0"))))))))

(fn IsValid
  (params (potentialLocation :type Vector))
  (return (not (Utilities|Set|Contains (Variables|Default|GetspawnedLocation) potentialLocation))))

(fn ToSpawn
  (return (<= (Math|Random|RandomFloatinRange 0.0 1.0) (Variables|Default|Getprobability))))

(fn SpawnFire
  (bind _locationtospawn (Variables|Default|GetlocationToSpawn))
  (LocalVariables|Setprevious _locationtospawn)
  (for _array_element (LocalVariables|Getprevious)
    (bind _location (CallFunction|GetFireLocation (+ (* _array_element (Variables|Default|Getlength)) (Variables|Default|Getorigin))))
    (bind _returnvalue (Game|SpawnActorfromClass "/Game/Weapon/Weapon_molotov/BP_Fire.BP_Fire_C" (Math|Conversions|ToTransform(Vector) _location) "Undefined" 0 0))
    (Default|SetTime _returnvalue 1.0)
    (CallFunction|GetPotentialSpawnPoint _array_element)
    (Utilities|Array|RemoveItem _locationtospawn _array_element)
    (Variables|Default|Setprobability (- (Variables|Default|Getprobability) 0.001))))

(fn GetFireLocation
  (params (xy :type Vector))
  (bind _outhit (Collision|LineTraceByChannel (Math|Vector|MakeVector (.x xy) (.y xy) 1e+04) (Math|Vector|MakeVector (.x xy) (.y xy) -1e+04) "TraceTypeQuery1" false 0 "None"))
  (return (.location _outhit)))