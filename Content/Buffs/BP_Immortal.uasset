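; BP_Immortal is a spinning buff pickup that makes the Bob character immune to damage for ten seconds.
; Tick adds a fixed rotation each frame, not scaled by delta time.
; On Box overlap with Bob it clears CanBeDamaged, plays a sound and destroys its box and mesh, staying alive through a Delay to restore the flag before destroying itself.
; An emissive material change on Bob is left unconnected.
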(event OnComponentBeginOverlap(Box)
  (params (OverlappedComponent :type Primitive%20Component%20Object%20Reference) (OtherActor :type Actor%20Object%20Reference) (OtherComp :type Primitive%20Component%20Object%20Reference) (OtherBodyIndex :type Integer) (bFromSweep :type Boolean) (SweepResult :type Hit%20Result%20Structure%20%28by%20ref%29))
  (bind _asbob (Utilities|Casting|CastToBob OtherActor))
  (Variables|/Script/Engine.Actor|SetbCanBeDamaged _asbob false)
  (Audio|PlaySound2D "/Game/Buffs/buff_sound.buff_sound" 1.0 1.0 0.0 0 0)
  (Components|DestroyComponent (Variables|Default|GetBox))
  (Utilities|FlowControl|Delay 1e+01)
  (Variables|/Script/Engine.Actor|SetbCanBeDamaged _asbob true)
  (Actor|DestroyActor))

(event EventBeginPlay)

(event Collision|EventActorBeginOverlap
  (params (OtherActor :type Actor%20Object%20Reference)))

(event EventTick
  (params (DeltaSeconds :type Float%20%28single-precision%29))
  (Transformation|AddActorLocalRotation "0,1.000000, 0" false false))

(fn ConstructionScript)