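; BP_Buff is a rotating pickup that applies a buff when a Bob overlaps its box, either for free or as a shop purchase.
; Shop items require enough coins and deduct the price from Bob's coin count before calling PerformBuff; other items call it directly.
; PerformBuff is an empty hook here, and the actor does not destroy or disable itself after use.
; The spin is a fixed per-tick rotation, so its speed depends on frame rate.
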(event OnComponentBeginOverlap(Box)
  (params (OverlappedComponent :type Primitive%20Component%20Object%20Reference) (OtherActor :type Actor%20Object%20Reference) (OtherComp :type Primitive%20Component%20Object%20Reference) (OtherBodyIndex :type Integer) (bFromSweep :type Boolean) (SweepResult :type Hit%20Result%20Structure%20%28by%20ref%29))
  (bind _asbob (Utilities|Casting|CastToBob OtherActor))
  (if (Variables|Default|GetIsShopItem)
    (if (>= (Variables|/Game/Characters/Bob.Bob_C|GetCoinCount _asbob) (Variables|Default|GetPrice))
      (CallFunction|DeductCoins _asbob)
      (CallFunction|PerformBuff _asbob :!label _label))
    (else
      (goto _label))))

(event EventBeginPlay)

(event Collision|EventActorBeginOverlap
  (params (OtherActor :type Actor%20Object%20Reference)))

(event EventTick
  (params (DeltaSeconds :type Float%20%28single-precision%29))
  (Transformation|AddActorLocalRotation "0,1.000000, 0" false false))

(fn ConstructionScript)

(fn DeductCoins
  (params (BobREF :type Bob%20Object%20Reference))
  (Variables|/Game/Characters/Bob.Bob_C|SetCoinCount BobREF (- (Variables|/Game/Characters/Bob.Bob_C|GetCoinCount BobREF) (Variables|Default|GetPrice))))

(fn PerformBuff
  (params (BobREF :type Bob%20Object%20Reference)))