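; Base health buff pickup that spins every tick and permanently raises the Bob character's max health on overlap.
; The overlap also heals up to half the new maximum, widens the HUD health bar and plays a sound.
; It then removes its box and mesh, waits, re-enables damage on Bob and destroys itself.
; A MovetoRandomLocation event slides the pickup along a random horizontal direction using a timeline lerp.
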(event OnComponentBeginOverlap(Box)
  (params (OverlappedComponent :type Primitive%20Component%20Object%20Reference) (OtherActor :type Actor%20Object%20Reference) (OtherComp :type Primitive%20Component%20Object%20Reference) (OtherBodyIndex :type Integer) (bFromSweep :type Boolean) (SweepResult :type Hit%20Result%20Structure%20%28by%20ref%29))
  (bind _asbob (Utilities|Casting|CastToBob OtherActor))
  (bind _output_get (Variables|/Game/Characters/Bob.Bob_C|SetMaxHealth _asbob (+ (Variables|/Game/Characters/Bob.Bob_C|GetMaxHealth _asbob) 4e+01)))
  (Variables|/Game/Characters/Bob.Bob_C|SetHealth _asbob (Math|Float|Min(Float) (+ (Variables|/Game/Characters/Bob.Bob_C|GetHealth _asbob) (/ _output_get 2.0)) _output_get))
  (Class|CanvasPanelSlot|SetSize (Class|WidgetLayoutLibrary|SlotasCanvasSlot (Variables|/Game/HUD/HUD.HUD_C|GetHealthBar (Variables|/Game/Characters/Bob.Bob_C|GetHUD _asbob))) (+ (Class|CanvasPanelSlot|GetSize (Class|WidgetLayoutLibrary|SlotasCanvasSlot (Variables|/Game/HUD/HUD.HUD_C|GetHealthBar (Variables|/Game/Characters/Bob.Bob_C|GetHUD _asbob)))) "(X=40.000000,Y=0.000000)"))
  (Audio|PlaySound2D "/Game/Buffs/buff_sound.buff_sound" 1.0 1.0 0.0 0 0)
  (Components|DestroyComponent (Variables|Default|GetBox))
  (Utilities|FlowControl|Delay 1e+01)
  (Variables|/Script/Engine.Actor|SetbCanBeDamaged _asbob true)
  (Actor|DestroyActor))

(event EventBeginPlay)

(event Collision|EventActorBeginOverlap
  (params (OtherActor :type Actor%20Object%20Reference)))

(event EventTick
  (params (DeltaSeconds :type Float%20%28single-precision%29))
  (Transformation|AddActorLocalRotation "0,1.000000, 0" false false))

(event EventMovetoRandomLocation
  (params (Range :type Float%20%28single-precision%29))
  (Variables|Default|SetStartLocation (Transformation|GetActorLocation))
  (Variables|Default|SetEndLocation (+ (Variables|Default|GetStartLocation) (* (Class|KismetMathLibrary|VectorNormal2D (Math|Random|RandomUnitVector) 0.0001) Range)))
  (bind _newtrack_0 (Timeline|Timeline_0 PlayFromStart)
    (:Update
      (Transformation|SetActorLocation (Math|Vector|Lerp(Vector) (Variables|Default|GetStartLocation) (Variables|Default|GetEndLocation) _newtrack_0) false false))))

(fn ConstructionScript)