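; BP_Coffee is a healing buff that restores Bob's health.
; PerformBuff passes the Bob reference to the Heal event, which adds a large fixed amount of health, capped at MaxHealth.
; It then plays a 2D buff sound and destroys the actor; at full health nothing happens, so the coffee remains.
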(event Custom|Heal
  (params (BobREF :type Bob%20Object%20Reference))
  (bind _maxhealth (Variables|/Game/Characters/Bob.Bob_C|GetMaxHealth BobREF))
  (if (not (>= (Variables|/Game/Characters/Bob.Bob_C|GetHealth BobREF) _maxhealth))
    (Variables|/Game/Characters/Bob.Bob_C|SetHealth BobREF (Math|Float|Min(Float) (+ (Variables|/Game/Characters/Bob.Bob_C|GetHealth BobREF) 1e+03) _maxhealth))
    (Audio|PlaySound2D "/Game/Buffs/buff_sound.buff_sound" 1.0 1.0 0.0 0 0)
    (Actor|DestroyActor)))

(event EventBeginPlay)

(event Collision|EventActorBeginOverlap
  (params (OtherActor :type Actor%20Object%20Reference)))

(fn ConstructionScript)

(fn PerformBuff
  (params (BobREF :type Bob%20Object%20Reference))
  (CallFunction|Heal BobREF))