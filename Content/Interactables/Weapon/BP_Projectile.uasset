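; Throwable physics projectile weapon that previews its arc while aiming and launches its item mesh when shot.
; Aiming rebuilds a spline from a predicted projectile path and lays temporary spline mesh components along it, cleared on stop or shoot.
; Preview and shot share one launch vector, tilted by an angle and scaled by strength and inverse mass relative to a benchmark.
; Damage passes to the parent only while the projectile is off the ground.
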(event EventBeginPlay
  (|CallParentFunction))

(event Collision|EventActorBeginOverlap
  (params (OtherActor :type Actor%20Object%20Reference)))

(event EventSetCollisionDisabled
  (Physics|SetSimulatePhysics (Variables|Default|GetItem%20Mesh) false)
  (|CallParentFunction))

(event EventTick
  (params (DeltaSeconds :type Float%20%28single-precision%29)))

(event EventStopAim
  (CallFunction|StopAim))

(event EventSetAim
  (params (location :type Vector :default "0, 0, 0") (direction :type Vector :default "0, 0, 0") (actors%20to%20ignore :type Array%20of%20Actor%20Object%20References))
  (CallFunction|Aim location direction actors%20to%20ignore))

(event EventShoot
  (params (direction :type Vector :default "0, 0, 0"))
  (CallFunction|ShootProjectile direction))

(fn ConstructionScript)

(fn Aim
  (params (location :type Vector) (direction :type Vector) (actos%20to%20ignore :type Array%20of%20Actor%20Object%20References))
  (CallFunction|GenerateSplinePoints location direction actos%20to%20ignore)
  (CallFunction|GenerateCurve))

(fn GenerateSplinePoints
  (params (location :type Vector) (direction :type Vector) (actors%20to%20ignore :type Array%20of%20Actor%20Object%20References))
  (CallFunction|ClearSplinePoints)
  (bind _launch_vector (CallFunction|GetLaunchVector direction))
  (bind _outpathpositions (Class|GameplayStatics|BlueprintPredictProjectilePathbyTraceChannel location _launch_vector true 0.0 "ECC_WorldStatic" true actors%20to%20ignore "None" 0.0 1e+01 3.0))
  (for (_array_element _array_index) _outpathpositions
    (Spline|AddSplinePointatIndex (Variables|Default|GetSpline) _array_element _array_index "Local" true))
  (Variables|Default|SetendPoint (Utilities|Array|Get(acopy) _outpathpositions (- (Utilities|Array|Length _outpathpositions) 1))))

(fn GenerateCurve
  (bind _spline (Variables|Default|GetSpline))
  (for _index (range 0 (- (Spline|GetNumberOfSplinePoints _spline) 1))
    (bind _returnvalue (AddComponent|AddSplineMeshComponent true))
    (Utilities|Array|Add (Variables|Default|Getspline%20meshes) _returnvalue)
    (SplineMesh|SetStartandEnd _returnvalue (.Location (Spline|GetLocationandTangentatSplinePoint _spline _index "Local")) (.Tangent (Spline|GetLocationandTangentatSplinePoint _spline _index "Local")) (.Location (Spline|GetLocationandTangentatSplinePoint _spline (+ _index 1) "Local")) (.Tangent (Spline|GetLocationandTangentatSplinePoint _spline (+ _index 1) "Local")) true :!class /Script/Engine.SplineMeshComponent)))

(fn StopAim
  (CallFunction|ClearSplinePoints))

(fn ClearSplinePoints
  (bind _spline_meshes (Variables|Default|Getspline%20meshes))
  (Spline|ClearSplinePoints (Variables|Default|GetSpline) true)
  (for _array_element _spline_meshes
    (Components|DestroyComponent _array_element))
  (Utilities|Array|Clear _spline_meshes))

(fn GetLaunchVector
  (params (Forward%20Direction :type Vector))
  (return (* (Math|Vector|Normalize (Math|Vector|RotateVectorAroundAxis Forward%20Direction (Variables|Default|Getangle) (Math|Vector|RotateVectorAroundAxis Forward%20Direction 9e+01 "0.000000,0.000000,1.000000"))) (* (/ (Variables|Default|GetBench%20Mark%20Mass) (Variables|Default|GetMass)) (Variables|Default|Getstrength)))))

(fn ShootProjectile
  (params (direction :type Vector))
  (bind _item_mesh (Variables|Default|GetItem%20Mesh))
  (CallFunction|ClearSplinePoints)
  (bind _launch_vector (CallFunction|GetLaunchVector direction))
  (Collision|SetCollisionEnabled _item_mesh "QueryAndPhysics")
  (Physics|SetSimulatePhysics _item_mesh true)
  (Class|PrimitiveComponent|SetAllPhysicsLinearVelocity _item_mesh _launch_vector false)
  (Class|PrimitiveComponent|SetAllPhysicsAngularVelocityinDegrees _item_mesh _launch_vector false))

(fn DealDamage
  (params (hit%20actor :type Actor%20Object%20Reference) (hit%20location :type Vector :default "0, 0, 0"))
  (bind _isonground (CallFunction|IsonGround))
  (if (not _isonground)
    (|CallParentFunction hit%20actor hit%20location)))

(fn SetMass
  (params (mass :type Float%20%28single-precision%29))
  (Variables|Default|SetMass mass))