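; BP_Interactable is a pickup item that outlines near the player and can be carried in a trolley.
; The outline uses custom depth with a rarity-based stencil, gated by readiness and trolley state on overlap, or set directly by trolley selection.
; Player overlap also freezes physics when a downward trace finds the item grounded.
; Dropping places it at given XY, restoring its initial rotation and height above the traced ground.
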(event EventTick
  (params (DeltaSeconds :type Float%20%28single-precision%29))
  (CallFunction|IsonGround))

(event Collision|EventActorBeginOverlap
  (params (OtherActor :type Actor%20Object%20Reference))
  (bind _item_mesh (Variables|Default|GetItem%20Mesh))
  (bind _isplayer (CallFunction|IsCollidingPlayer OtherActor))
  (if _isplayer
    (CallFunction|SetHighlight true)
    (bind _isonground (CallFunction|IsonGround))
    (if _isonground
      (Physics|SetSimulatePhysics _item_mesh false)
      (Collision|SetCollisionEnabled _item_mesh "QueryOnly"))))

(event EventSetCollisionEnabled
  (Collision|SetCollisionEnabled (Variables|Default|GetItem%20Mesh) "QueryOnly"))

(event EventSetCollisionDisabled
  (Collision|SetCollisionEnabled (Variables|Default|GetItem%20Mesh) "NoCollision"))

(event EventSelectinTrolley
  (CallFunction|Select))

(event EventBeginPlay
  (bind _item_mesh (Variables|Default|GetItem%20Mesh))
  (bind _returnvalue (Transformation|GetWorldLocation _item_mesh))
  (Variables|Default|SetLength (Components|Sphere|GetScaledSphereRadius (Variables|Default|GetSphere)))
  (bind _value (CallFunction|GetRarityValue))
  (Rendering|SetCustomDepthStencilValue (Variables|Default|GetItem%20Mesh) _value)
  (Variables|Default|Setoriginal%20rotation (Transformation|GetWorldRotation (Variables|Default|GetItem%20Mesh)))
  (bind _outhit (Collision|LineTraceByChannel _returnvalue (- _returnvalue "0, 0,10000.000000") "TraceTypeQuery1" false 0 "None"))
  (bind _output_get (Variables|Default|Setheight (- (.z (Transformation|GetWorldLocation (Variables|Default|GetItem%20Mesh))) (.z (.location _outhit))))))

(event EventDeselectinTrolley
  (CallFunction|Deselect))

(event EventDrop
  (params (bias :type Vector :default "0, 0, 0"))
  (CallFunction|DropItem bias))

(event Collision|EventActorEndOverlap
  (params (OtherActor :type Actor%20Object%20Reference))
  (bind _isplayer (CallFunction|IsCollidingPlayer OtherActor))
  (if _isplayer
    (CallFunction|SetHighlight false)))

(event EventToggleTrolley
  (CallFunction|ToggleinTrolley))

(event EventDelayReadytoHighlight
  (Utilities|FlowControl|Delay 0.5)
  (Variables|Default|SetisReadyToHighlight true))

(event EventSetHighlight
  (params (toHighlight :type Boolean))
  (CallFunction|SetHighlight toHighlight)
  (Variables|Default|SetisReadyToHighlight toHighlight))

(fn ConstructionScript)

(fn SetHighlight
  (params (toHighlight :type Boolean))
  (if toHighlight
    (if (Math|Boolean|ANDBoolean toHighlight (Variables|Default|GetisReadyToHighlight) (not (Variables|Default|GetisInTrolley)))
      (Rendering|SetRenderCustomDepth (Variables|Default|GetItem%20Mesh) toHighlight :!label _label))
    (else
      (goto _label))))

(fn ToggleinTrolley
  (Variables|Default|SetisInTrolley (not (Variables|Default|GetisInTrolley))))

(fn IsCollidingPlayer
  (params (actor :type Actor%20Object%20Reference))
  (return (Actor|ActorHasTag actor "player")))

(fn IsonGround
  (bind _sphere (Variables|Default|GetSphere))
  (bind _returnvalue (Transformation|GetWorldLocation _sphere))
  (bind _outhit (Collision|LineTraceByChannel _returnvalue (+ _returnvalue (Math|Vector|MakeVector 0.0 0.0 -1e+04)) "TraceTypeQuery1" false 0 "None"))
  (return (<= (Math|Vector|VectorLength (- (Transformation|GetWorldLocation (Variables|Default|GetSphere)) (.Location (Collision|BreakHitResult _outhit)))) (Variables|Default|GetLength))))

(fn Select
  (Rendering|SetRenderCustomDepth (Variables|Default|GetItem%20Mesh) true))

(fn Deselect
  (Rendering|SetRenderCustomDepth (Variables|Default|GetItem%20Mesh) false))

(fn GetRarityValue
  (return (.Value (Utilities|Map|Find (Variables|Default|GetRarityValueMapping) (Variables|Default|GetRarirty)))))

(fn DropItem
  (params (bias :type Vector))
  (bind _item_mesh (Variables|Default|GetItem%20Mesh))
  (bind _returnvalue (Transformation|GetWorldLocation _item_mesh))
  (LocalVariables|Setbyas bias)
  (bind _outhit (Collision|LineTraceByChannel _returnvalue (- _returnvalue "0, 0,10000.000000") "TraceTypeQuery1" false 0 "None" true "(R=0.000000,G=1.000000,B=0.984913,A=1.000000)" "(R=1.000000,G=0.000000,B=0.008142,A=1.000000)"))
  (Transformation|SetActorLocationAndRotation (Math|Vector|MakeVector (.x (LocalVariables|Getbyas)) (.y (LocalVariables|Getbyas)) (+ (.z (.location _outhit)) (Variables|Default|Getheight))) (Variables|Default|Getoriginal%20rotation)))

(fn GetLength
  (return (Variables|Default|GetLength)))