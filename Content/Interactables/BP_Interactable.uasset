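; BP_Interactable is an interactable item that toggles a custom-depth highlight when a player-tagged actor overlaps it.
; Highlighting turns on only when the item is ready and not in a trolley, with events for toggling trolley state, delayed readiness and mesh collision.
; A downward trace at BeginPlay records resting height; on player overlap, a repeat trace within that distance disables physics and sets collision to query-only.
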(event Collision|EventActorBeginOverlap
  (params (OtherActor :type Actor%20Object%20Reference))
  (bind _item_mesh (Variables|Default|GetItem%20Mesh))
  (bind _isplayer (CallFunction|IsCollidingPlayer OtherActor))
  (if _isplayer
    (CallFunction|SetHighlight true)
    (bind _isonground (CallFunction|IsonGround))
    (if _isonground
      (Physics|SetSimulatePhysics _item_mesh false)
      (Collision|SetCollisionEnabled _item_mesh "QueryOnly"))))

(event EventSetCollisionEnabled
  (Collision|SetCollisionEnabled (Variables|Default|GetItem%20Mesh) "QueryOnly"))

(event EventSetCollisionDisabled
  (Collision|SetCollisionEnabled (Variables|Default|GetItem%20Mesh) "NoCollision"))

(event EventTick
  (params (DeltaSeconds :type Float%20%28single-precision%29)))

(event EventBeginPlay
  (bind _sphere (Variables|Default|GetSphere))
  (bind _returnvalue (Transformation|GetWorldLocation _sphere))
  (bind _outhit (Collision|LineTraceByChannel _returnvalue (+ _returnvalue (Math|Vector|MakeVector 0.0 0.0 -1e+04)) "TraceTypeQuery1" false 0 "None"))
  (Variables|Default|SetLength (Math|Vector|VectorLength (- (Transformation|GetWorldLocation (Variables|Default|GetSphere)) (.location _outhit)))))

(event Collision|EventActorEndOverlap
  (params (OtherActor :type Actor%20Object%20Reference))
  (bind _isplayer (CallFunction|IsCollidingPlayer OtherActor))
  (if _isplayer
    (CallFunction|SetHighlight false)))

(event EventToggleTrolley
  (CallFunction|ToggleinTrolley))

(event EventDelayReadytoHighlight
  (Utilities|FlowControl|Delay 0.5)
  (Variables|Default|SetisReadyToHighlight true))

(event EventSetHighlight
  (params (toHighlight :type Boolean))
  (CallFunction|SetHighlight toHighlight)
  (Variables|Default|SetisReadyToHighlight toHighlight))

(fn ConstructionScript)

(fn SetHighlight
  (params (toHighlight :type Boolean))
  (if toHighlight
    (if (Math|Boolean|ANDBoolean toHighlight (Variables|Default|GetisReadyToHighlight) (not (Variables|Default|GetisInTrolley)))
      (Rendering|SetRenderCustomDepth (Variables|Default|GetItem%20Mesh) toHighlight :!label _label))
    (else
      (goto _label))))

(fn ToggleinTrolley
  (Variables|Default|SetisInTrolley (not (Variables|Default|GetisInTrolley))))

(fn IsCollidingPlayer
  (params (actor :type Actor%20Object%20Reference))
  (return (Actor|ActorHasTag actor "player")))

(fn IsonGround
  (bind _sphere (Variables|Default|GetSphere))
  (bind _returnvalue (Transformation|GetWorldLocation _sphere))
  (bind _outhit (Collision|LineTraceByChannel _returnvalue (+ _returnvalue (Math|Vector|MakeVector 0.0 0.0 -1e+04)) "TraceTypeQuery1" false 0 "None"))
  (return (<= (Math|Vector|VectorLength (- (Transformation|GetWorldLocation (Variables|Default|GetSphere)) (.Location (Collision|BreakHitResult _outhit)))) (Variables|Default|GetLength))))