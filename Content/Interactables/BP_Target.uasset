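; BP_Target is an interactable target that detects hits from attacking BP_Weapon actors on overlap.
; On overlap it passes the weapon and its damage to RecieveDamage, which stores a timestamp per weapon in the References map.
; A repeat hit from the same weapon refreshes that timestamp only after TimeReady seconds have elapsed, acting as a per-weapon cooldown.
; Damage is not applied, and the debug prints are disconnected.
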(event EventBeginPlay)

(event Collision|EventActorBeginOverlap
  (params (OtherActor :type Actor%20Object%20Reference))
  (bind _asbp_weapon (Utilities|Casting|CastToBP_Weapon OtherActor))
  (bind _is_attacking (Default|GetIsAttacking _asbp_weapon))
  (if _is_attacking
    (bind _damage (Default|GetDamage _asbp_weapon))
    (CallFunction|RecieveDamage _damage _asbp_weapon)))

(event EventTick
  (params (DeltaSeconds :type Float%20%28single-precision%29)))

(fn ConstructionScript)

(fn CheckReady
  (params (dateTime :type Date%20Time%20Structure))
  (return (< (LocalVariables|GettimeReady) (Math|Timespan|GetSeconds (- (Math|DateTime|Now) dateTime)))))

(fn RecieveDamage
  (params (damage :type Float%20%28single-precision%29) (weapon :type BP%20Weapon%20Object%20Reference))
  (bind _references (Variables|Default|GetReferences))
  (bind (_value _returnvalue) (Utilities|Map|Find _references weapon))
  (if (not _returnvalue)
    (Utilities|Map|Add (Variables|Default|GetReferences) weapon (Math|DateTime|Now) :!label _label)
    (else
      (bind _ready (CallFunction|CheckReady _value))
      (if _ready
        (goto _label)))))