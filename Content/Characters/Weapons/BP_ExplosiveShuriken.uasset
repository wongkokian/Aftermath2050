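; BP_ExplosiveShuriken is an explosive shuriken weapon whose damage comes from its explosion rather than direct hits.
; On BeginPlay it configures mass, attack range and damage through setters, zeroing regular damage and enabling explosive damage.
; ActivateCollision switches its Box to an overlap-all profile, and DeactivateCollision disables that collision.
; The Blueprint contains no overlap or detonation logic of its own.
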(event EventBeginPlay
  (CallFunction|SetMass 4e+01)
  (CallFunction|SetAttackRange 6e+02)
  (CallFunction|SetDamage 0.0)
  (CallFunction|SetExplosive true)
  (CallFunction|SetExplosiveDamage 3e+01))

(event Collision|EventActorBeginOverlap
  (params (OtherActor :type Actor%20Object%20Reference)))

(event EventTick
  (params (DeltaSeconds :type Float%20%28single-precision%29)))

(event EventDeactivateCollision
  (Collision|SetCollisionEnabled (Variables|Default|GetBox) "NoCollision"))

(event EventActivateCollision
  (Collision|SetCollisionProfileName (Variables|Default|GetBox) "OverlapAll" true :!class /Script/Engine.PrimitiveComponent))

(fn ConstructionScript)