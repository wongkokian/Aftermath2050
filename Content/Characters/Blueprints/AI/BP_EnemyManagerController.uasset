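; AI controller for the enemy manager that runs the BT_EnemyManager behavior tree on BeginPlay.
; It then calls OnBobEnters, a step noted as used in the test stage, to seed the blackboard.
; That event registers the controller as EnemyManager, then after a short delay stores the player character and flags the player as alive.
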(event Custom|OnBobEnters
  ;[1 1 1] Assign self as the EnemyManager in blackboard BB_stage
  (AI|Components|Blackboard|SetValueasObject (Variables|Default|GetBlackboard) (Utilities|Name|MakeLiteralName "EnemyManager") self)
  (Utilities|FlowControl|Delay 0.2)
  (AI|Components|Blackboard|SetValueasObject (Variables|Default|GetBlackboard) (Utilities|Name|MakeLiteralName "PlayerActor") (Game|GetPlayerCharacter 0))
  (AI|Components|Blackboard|SetValueasBool (Variables|Default|GetBlackboard) (Utilities|Name|MakeLiteralName "IsPlayerAlive") true))

(event EventBeginPlay
  (AI|RunBehaviorTree "/Game/Characters/Blueprints/AI/BT_EnemyManager.BT_EnemyManager")
  ;[1 1 1] Used in test stage
  (CallFunction|OnBobEnters))

(fn ConstructionScript)