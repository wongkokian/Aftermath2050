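; Behavior tree task that writes a new strafe location for the AI-controlled pawn to a blackboard vector key.
; The point is the pawn's location plus its forward vector and its right vector weighted three times, randomly left or right, all scaled by GetDistance.
; GetDistance holds a random min-to-max distance calculation, but that result is left unconnected.
; The task finishes successfully right after writing the key.
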(event EventReceiveExecuteAI
  (params (OwnerController :type AI%20Controller%20Object%20Reference) (ControlledPawn :type Pawn%20Object%20Reference))
  (bind _number (CallFunction|3or-3))
  (AI|BehaviorTree|SetBlackboardValueasVector (Variables|Default|GetKey) (+ (* (+ (* (Transformation|GetActorRightVector ControlledPawn) _number) (Transformation|GetActorForwardVector ControlledPawn)) (Utilities|GetDistance)) (Transformation|GetActorLocation ControlledPawn)))
  (AI|BehaviorTree|FinishExecute true))

(fn 3or-3
  (if (Math|Random|RandomBool)
    (return 3.0)
    (else
      (return -3.0))))