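; AI controller for the slow zombie that runs the BT_Slowzombie behavior tree on begin play.
; Hit and death events feed the tree through Blackboard booleans, with death clearing IsAlive.
; The hit handler branches between the IsHit and IsHit_2 flags, but its condition is fixed at true, so it always sets IsHit_2 and clears IsHit.
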(event Custom|On%20Hit
  (bind _blackboard (Variables|Default|GetBlackboard))
  (bind _blackboard_2 (Variables|Default|GetBlackboard))
  (if true
    (AI|Components|Blackboard|SetValueasBool _blackboard_2 (Utilities|Name|MakeLiteralName "IsHit_2") true)
    (AI|Components|Blackboard|SetValueasBool _blackboard (Utilities|Name|MakeLiteralName "IsHit") false)
    (else
      (AI|Components|Blackboard|SetValueasBool _blackboard_2 (Utilities|Name|MakeLiteralName "IsHit") true)
      (AI|Components|Blackboard|SetValueasBool _blackboard (Utilities|Name|MakeLiteralName "IsHit_2") false))))

(event Custom|On%20Killed
  (AI|Components|Blackboard|SetValueasBool (Variables|Default|GetBlackboard) (Utilities|Name|MakeLiteralName "IsAlive") false))

(event EventBeginPlay
  (AI|RunBehaviorTree "/Game/Characters/Blueprints/AI/BT_Slowzombie.BT_Slowzombie"))

(event EventTick
  (params (DeltaSeconds :type Float%20%28single-precision%29)))

(fn ConstructionScript)