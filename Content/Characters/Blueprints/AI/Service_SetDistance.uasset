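; Behavior tree service that tracks how far an AI character is from the player for combat decisions.
; Each tick it measures the distance from the controlled pawn to the PlayerLocation blackboard vector and writes it to DistanceToPlayer.
; It also compares that distance against attack and strafe range thresholds to set the IsInAttackRange and IsInStrafeRange blackboard flags.
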(event EventReceiveTickAI
  (params (OwnerController :type AI%20Controller%20Object%20Reference) (ControlledPawn :type Pawn%20Object%20Reference) (DeltaSeconds :type Float%20%28single-precision%29))
  (bind _returnvalue (Transformation|GetActorLocation ControlledPawn))
  (bind _playerlocation (Variables|Default|GetPlayerLocation))
  (bind _returnvalue_2 (Class|BTFunctionLibrary|GetBlackboardValueasVector _playerlocation))
  (bind _returnvalue_3 (Math|Vector|Distance(Vector) _returnvalue _returnvalue_2))
  (Class|BTFunctionLibrary|SetBlackboardValueasFloat (Variables|Default|GetDistanceToPlayer) _returnvalue_3)
  (Class|BTFunctionLibrary|SetBlackboardValueasBool (Variables|Default|GetIsInAttackRange) (< _returnvalue_3 (Variables|Default|GetAttackRange)))
  (Class|BTFunctionLibrary|SetBlackboardValueasBool (Variables|Default|GetIsInStrafeRange) (< _returnvalue_3 (Variables|Default|GetStrafeRange))))