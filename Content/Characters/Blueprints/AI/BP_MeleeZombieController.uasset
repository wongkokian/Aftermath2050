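; AI controller for the melee zombie that runs the BT_MeleeZombie behavior tree on begin play and passes combat events to its Blackboard.
; OnHit sets one of the IsHit and IsHit_2 flags and clears the other, branching on GetBbIsHit, whose graph holds only an unused Blackboard read.
; OnKilled sets IsAlive to false.
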(event Custom|OnKilled
  (AI|Components|Blackboard|SetValueasBool (Variables|Default|GetBlackboard) (Utilities|Name|MakeLiteralName "IsAlive") false))

(event Custom|OnHit
  (bind _blackboard (Variables|Default|GetBlackboard))
  (bind _blackboard_2 (Variables|Default|GetBlackboard))
  (if (Utilities|GetBbIsHit)
    (AI|Components|Blackboard|SetValueasBool _blackboard_2 (Utilities|Name|MakeLiteralName "IsHit_2") true)
    (AI|Components|Blackboard|SetValueasBool _blackboard (Utilities|Name|MakeLiteralName "IsHit") false)
    (else
      (AI|Components|Blackboard|SetValueasBool _blackboard_2 (Utilities|Name|MakeLiteralName "IsHit") true)
      (AI|Components|Blackboard|SetValueasBool _blackboard (Utilities|Name|MakeLiteralName "IsHit_2") false))))

(event EventBeginPlay
  (AI|RunBehaviorTree "/Game/Characters/Blueprints/AI/BT_MeleeZombie.BT_MeleeZombie"))

(fn ConstructionScript)