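; BP_MeleeZombie is the melee zombie character, handling its health, damage reactions and walk speed.
; BeginPlay caches the anim blueprint and checks for a zombie controller, but sets AiController to None instead of the cast result.
; AnyDamage subtracts Health, then notifies AiController of a hit or kill, clearing the anim blueprint's IsAlive on death.
; SetSpeed drives MaxWalkSpeed; the string built inside GetDamageString for debug printing is unused.
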(event Custom|SetSpeed
  (params (Speed :type Float%20%28single-precision%29))
  (Variables|/Script/Engine.CharacterMovementComponent|SetMaxWalkSpeed (Variables|Character|GetCharacterMovement) Speed))

(event EventBeginPlay
  (bind _asmelee_zombie_anim_bp (Utilities|Casting|CastToMeleeZombie_AnimBP (Components|SkeletalMesh|GetAnimInstance (Variables|Character|GetMesh)))
    (:then
      (Variables|Default|SetAnimBP _asmelee_zombie_anim_bp)
      (Utilities|Casting|CastToBP_MeleeZombieController (Pawn|GetController)
        (:then
          (Variables|Default|SetAiController 0))
        (:CastFailed
          (Development|PrintString "cast failed: zombie controller"))))
    (:CastFailed
      (Development|PrintString "cast failed: zombie anim bp "))))

(event Game|Damage|EventAnyDamage
  (params (Damage :type Float%20%28single-precision%29) (DamageType :type Damage%20Type%20Object%20Reference) (InstigatedBy :type Controller%20Object%20Reference) (DamageCauser :type Actor%20Object%20Reference))
  (bind _aicontroller (Variables|Default|GetAiController))
  (Variables|Default|SetHealth (- (Variables|Default|GetHealth) Damage))
  (Development|PrintString (Utilities|GetDamageString Damage))
  (if (> (Variables|Default|GetHealth) 0.0)
    (Default|OnHit _aicontroller)
    (else
      (Default|OnKilled _aicontroller)
      (Variables|/Game/Characters/Animations/MeleeZombie_AnimBP.MeleeZombie_AnimBP_C|SetIsAlive (Variables|Default|GetAnimBP) false))))

(fn ConstructionScript)