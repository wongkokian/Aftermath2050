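; Boss ninja character that throws random shurikens at the player, with an occasional explosive one on cooldown, and drives the player HUD's boss health bar.
; Each tick a line trace to the player reports blocked sight to BP_NinjaController, which also receives hit and death notifications.
; Rapid hits trigger timed, glowing hyperarmour that suppresses hit reactions and knockback.
; Also provides teleport near the player, lock-on marker and slow-motion kill cam.
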(event Custom|SetSpeed
  (params (Speed :type Float%20%28single-precision%29))
  (Variables|/Script/Engine.CharacterMovementComponent|SetMaxWalkSpeed (Variables|Character|GetCharacterMovement) Speed))

(event Custom|HyperarmourCountdown
  (Utilities|FlowControl|DoOnce false :!label _label
    (:Completed
      (Rendering|Material|SetScalarParameterValueonMaterials (Variables|Character|GetMesh) "EmissiveColor" 1.0)
      (Utilities|FlowControl|Delay (Variables|Default|GetHyperarmourTime))
      (CallFunction|ResetHitCount)
      (Variables|Default|SetIsHyperarmour false)
      (Rendering|Material|SetScalarParameterValueonMaterials (Variables|Character|GetMesh) "EmissiveColor" 0.0)
      (goto _label Reset))))

(event Custom|Set%20Speed
  (params (Speed :type Float%20%28single-precision%29))
  (Variables|/Script/Engine.CharacterMovementComponent|SetMaxWalkSpeed (Variables|Character|GetCharacterMovement) Speed))

(event Custom|Shoot
  (Utilities|ShootProjectile)
  (Utilities|FlowControl|Delay 2.0)
  (if (Variables|Default|GetIsInCooldown)
    (bind _weapontype (CallFunction|RandomWeapon))
    (CallFunction|SpawnWeapon _weapontype)
    (elif (Math|Random|RandomBoolwithWeight 0.4)
      (bind _weapontype_2 (CallFunction|RandomWeapon))
      (CallFunction|SpawnWeapon _weapontype_2)
      (else
        (CallFunction|SpawnWeapon "/Game/Characters/Weapons/BP_ExplosiveShuriken.BP_ExplosiveShuriken_C")
        (Variables|Default|SetIsInCooldown true)
        (Utilities|FlowControl|Delay 1e+01)
        (Variables|Default|SetIsInCooldown false)))))

(event EventBeginPlay
  (CallFunction|Init)
  (bind _weapontype (CallFunction|RandomWeapon))
  (CallFunction|SpawnWeapon _weapontype)
  (Variables|Default|SetAttack%20Range (Variables|/Game/Characters/Weapons/EnemyProjectile.EnemyProjectile_C|GetAttackRange (Variables|Default|GetHeld%20Item))))

(event Game|Damage|EventAnyDamage
  (params (Damage :type Float%20%28single-precision%29) (DamageType :type Damage%20Type%20Object%20Reference) (InstigatedBy :type Controller%20Object%20Reference) (DamageCauser :type Actor%20Object%20Reference))
  (bind _aicontroller (Variables|Default|GetAiController))
  (bind _output_get (Variables|Default|SetHealth (- (Variables|Default|GetHealth) Damage)))
  (bind _asbob (Utilities|Casting|CastToBob (Game|GetPlayerCharacter 0)))
  (Variables|/Game/HUD/HUD.HUD_C|SetBossHealth (Variables|/Game/Characters/Bob.Bob_C|GetHUD _asbob) _output_get)
  (CallFunction|SetHitCount)
  (if (> (Variables|Default|GetHealth) 0.0)
    (if (Variables|Default|GetIsHyperarmour)
      (CallFunction|HyperarmourCountdown)
      (else
        (Default|OnHit _aicontroller)
        (Animation|PlayAnimMontage "/Game/Characters/Animations/Ninja/Ninja_Reaction_Hit_Short.Ninja_Reaction_Hit_Short" 1.0 "None")
        (Physics|AddImpulse (Variables|Character|GetCharacterMovement) (Utilities|GetHitImpulse (Game|Player|GetPlayerPawn 0) (Variables|Default|GetHitImpulse)) true)))
    (else
      (Default|OnKilled _aicontroller)
      (Variables|/Game/Characters/Animations/Ninja/Ninja_AnimBP.Ninja_AnimBP_C|SetIsAlive (Variables|Default|GetAnimBP) false)
      (Variables|/Game/HUD/HUD.HUD_C|SetBossBarVisibility (Variables|/Game/Characters/Bob.Bob_C|GetHUD _asbob) "Hidden")
      (Variables|/Game/HUD/HUD.HUD_C|SetBossNameVisibility (Variables|/Game/Characters/Bob.Bob_C|GetHUD _asbob) "Hidden"))))

(event EventKillCam
  (CallFunction|ChooseCamera)
  (CallFunction|ChangeCamera)
  (Utilities|Time|SetGlobalTimeDilation 0.5)
  (Utilities|FlowControl|Delay 2.0)
  (Utilities|Time|SetGlobalTimeDilation 1.0)
  (CallFunction|ChangeCameraBack))

(event EventShowLockSpot
  (Development|SetHiddeninGame (Variables|Default|GetLockSpot) false false))

(event EventHideLockSpot
  (Development|SetHiddeninGame (Variables|Default|GetLockSpot) true false))

(event EventTick
  (params (DeltaSeconds :type Float%20%28single-precision%29))
  (bind _aicontroller (Variables|Default|GetAiController))
  (bind _isblock (CallFunction|IsBlock))
  (if _isblock
    (Default|OnBlocked _aicontroller)
    (else
      (Default|OnNotBlocked _aicontroller))))

(event Collision|EventActorBeginOverlap
  (params (OtherActor :type Actor%20Object%20Reference)))

(fn ConstructionScript)

(fn Init
  (bind _asninja_anim_bp (Utilities|Casting|CastToNinja_AnimBP (Components|SkeletalMesh|GetAnimInstance (Variables|Character|GetMesh))))
  (Variables|Default|SetAnimBP _asninja_anim_bp)
  (bind _asbp_ninja_controller (Utilities|Casting|CastToBP_NinjaController (Pawn|GetController)))
  (Variables|Default|SetAiController _asbp_ninja_controller))

(fn IsBlock
  (bind _returnvalue (Collision|LineTraceByChannel (Transformation|GetActorLocation) (Transformation|GetWorldLocation (Variables|/Script/Engine.Character|GetCapsuleComponent (Game|GetPlayerCharacter 0))) "TraceTypeQuery1" false 0 "None"))
  (return _returnvalue))

(fn SpawnWeapon
  (params (Weapon%20Type :type Actor%20Class%20Reference))
  (bind _returnvalue (Game|SpawnActorfromClass Weapon%20Type (Transformation|GetSocketTransform (Variables|Character|GetMesh) "ShurikenSocket" "RTS_World") "AlwaysSpawn" 0 0))
  (bind _asenemy_projectile (Utilities|Casting|CastToEnemyProjectile _returnvalue))
  (Class|IWeapon|DeactivateCollision(Message) _asenemy_projectile)
  (Transformation|AttachComponentToComponent _asenemy_projectile (Variables|Character|GetMesh) "ShurikenSocket" "SnapToTarget" "SnapToTarget" "SnapToTarget" true)
  (Variables|Default|SetHeld%20Item _asenemy_projectile)
  (Variables|Default|SetIsHolding true))

(fn ChangeCamera
  (Game|Player|SetViewTargetwithBlend (Game|GetPlayerController 0) (Components|GetOwner (Variables|Default|GetCamera)) 0.0 "VTBlend_Linear" 0.0 false))

(fn ChangeCameraBack
  (bind _asbob (Utilities|Casting|CastToBob (Game|GetPlayerCharacter 0)))
  (Game|Player|SetViewTargetwithBlend (Game|GetPlayerController 0) (Components|GetOwner (Variables|/Game/Characters/Bob.Bob_C|GetFollowCamera _asbob)) 0.0 "VTBlend_Linear" 0.0 false))

(fn ChooseCamera
  (bind _camera (Variables|Default|GetCamera))
  (bind _camera1 (Variables|Default|GetCamera1))
  (bind _returnvalue (Collision|LineTraceByChannel (Transformation|GetWorldLocation (Variables|Default|GetCamera)) (Transformation|GetWorldLocation (Variables|/Script/Engine.Character|GetCapsuleComponent (Game|GetPlayerCharacter 0))) "TraceTypeQuery1" false 0 "None"))
  (if _returnvalue
    (Components|Activation|SetActive _camera false true)
    (Components|Activation|SetActive _camera1 true false)
    (else
      (Components|Activation|SetActive _camera true false)
      (Components|Activation|SetActive _camera1 false true))))

(fn Teleport
  (Audio|SpawnSoundatLocation "/Game/Characters/Audio/Ninja_Teleport_sound.Ninja_Teleport_sound" (Transformation|GetActorLocation) "0, 0, 0" 1.0 1.0 0.0 0 0)
  (Transformation|SetActorLocation (+ (.RandomLocation (AI|Navigation|GetRandomReachablePointinRadius (Transformation|GetWorldLocation (Variables|/Script/Engine.Character|GetCapsuleComponent (Game|GetPlayerCharacter 0))) 6e+02 0 0)) (Math|Vector|MakeVector 0.0 0.0 88.0)) false false))

(fn RandomWeapon
  (bind _shurikentype (Variables|Default|GetShurikenType))
  (return (Utilities|Array|Get(acopy) _shurikentype (Math|Random|RandomInteger (Utilities|Array|Length _shurikentype)))))

(fn SetHitCount
  (bind _returnvalue (Actor|GetGameTimeSinceCreation))
  (if (not (Variables|Default|GetIsHyperarmour))
    (if (> (- _returnvalue (Variables|Default|GetHitTime)) (Variables|Default|GetResetTime))
      (CallFunction|ResetHitCount)
      (Variables|Default|SetHitTime _returnvalue))
    (bind _result (Math|Integer|IncrementInt (Variables|Default|GetHitCount))
      (:%20%20
        (if (not (< _result (Variables|Default|GetHitLimit)))
          (Variables|Default|SetIsHyperarmour true))))))

(fn ResetHitCount
  (Variables|Default|SetHitTime 0.0)
  (Variables|Default|SetHitCount 0))

(fn IsAlive
  (return (> (Variables|Default|GetHealth) 0.0)))