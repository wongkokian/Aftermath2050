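; BP_FizzFire is a short-lived fire hazard from Fizz's weapon set that damages Bob.
; On BeginPlay it spawns a scaled-down fire particle at its collision box, waits for Time (settable through SetTime), then destroys the particle and itself.
; Box overlaps call DealDamage, which applies damage only to an actor whose class is exactly Bob, and only once per fire via the HasHit flag.
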(event OnComponentBeginOverlap(Box)
  (params (OverlappedComponent :type Primitive%20Component%20Object%20Reference) (OtherActor :type Actor%20Object%20Reference) (OtherComp :type Primitive%20Component%20Object%20Reference) (OtherBodyIndex :type Integer) (bFromSweep :type Boolean) (SweepResult :type Hit%20Result%20Structure%20%28by%20ref%29))
  (CallFunction|DealDamage OtherActor (.impactpoint SweepResult)))

(event EventBeginPlay
  (bind _returnvalue (Effects|SpawnEmitteratLocation "/Game/Realistic_Starter_VFX_Pack_Vol2/Particles/Fire/P_Fire_Big.P_Fire_Big" (Transformation|GetWorldLocation (Variables|Default|GetBox)) "0, 0, 0" "0.100000,0.100000,0.100000"))
  (Variables|Default|Setfire%20particle _returnvalue)
  (Utilities|FlowControl|Delay (Variables|Default|Gettime))
  (Components|DestroyComponent (Variables|Default|Getfire%20particle))
  (Actor|DestroyActor))

(event Collision|EventActorBeginOverlap
  (params (OtherActor :type Actor%20Object%20Reference)))

(event EventTick
  (params (DeltaSeconds :type Float%20%28single-precision%29)))

(fn ConstructionScript)

(fn SetTime
  (params (duration :type Float%20%28single-precision%29))
  (Variables|Default|Settime duration))

(fn DealDamage
  (params (hit%20actor :type Actor%20Object%20Reference) (hit%20location :type Vector))
  (if (and (== (Utilities|GetClass hit%20actor) "/Game/Characters/Bob.Bob_C") (not (Variables|Default|GetHas%20Hit)))
    (Variables|Default|SetHas%20Hit true)
    (Game|Damage|ApplyDamage hit%20actor (Variables|Default|GetDamage) 0 self)))