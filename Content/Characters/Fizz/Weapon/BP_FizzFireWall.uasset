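; BP_FizzFireWall is a short-lived fire wall weapon actor for the Fizz character that damages Bob.
; On BeginPlay it plays an explosion sound at its location and sets a brief life span.
; Its Sphere overlap applies fixed damage only to actors of exactly the Bob class, with a HasHit flag limiting each wall to a single hit.
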(event OnComponentBeginOverlap(Sphere)
  (params (OverlappedComponent :type Primitive%20Component%20Object%20Reference) (OtherActor :type Actor%20Object%20Reference) (OtherComp :type Primitive%20Component%20Object%20Reference) (OtherBodyIndex :type Integer) (bFromSweep :type Boolean) (SweepResult :type Hit%20Result%20Structure%20%28by%20ref%29))
  (if (and (== (Utilities|GetClass OtherActor) "/Game/Characters/Bob.Bob_C") (not (Variables|Default|GetHas%20Hit)))
    (Variables|Default|SetHas%20Hit true)
    (Game|Damage|ApplyDamage OtherActor 1e+01 0 self)))

(event EventBeginPlay
  (Audio|PlaySoundatLocation "/Game/Characters/Audio/Explosion_sound.Explosion_sound" (Transformation|GetActorLocation) "0, 0, 0" 1.0 1.0 0.0 0 0 0)
  (Actor|SetLifeSpan 2.0))

(event Collision|EventActorBeginOverlap
  (params (OtherActor :type Actor%20Object%20Reference)))

(event EventTick
  (params (DeltaSeconds :type Float%20%28single-precision%29)))

(fn ConstructionScript)