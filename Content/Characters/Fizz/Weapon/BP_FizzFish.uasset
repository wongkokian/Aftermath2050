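; Fizz's fish weapon, a physics-launched projectile that damages Bob on overlap and plays a frying sound on spawn.
; ShootProjectile enables box overlap and mesh physics, then sets linear and angular velocity from a pitched direction scaled inversely by mass.
; The first Box overlap with Bob applies damage, plays an impact sound and destroys the fish.
; Any blocking hit also plays the sound and destroys it.
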(event OnComponentBeginOverlap(Box)
  (params (OverlappedComponent :type Primitive%20Component%20Object%20Reference) (OtherActor :type Actor%20Object%20Reference) (OtherComp :type Primitive%20Component%20Object%20Reference) (OtherBodyIndex :type Integer) (bFromSweep :type Boolean) (SweepResult :type Hit%20Result%20Structure%20%28by%20ref%29))
  (if (and (== (Utilities|GetClass OtherActor) "/Game/Characters/Bob.Bob_C") (not (Variables|Default|GetHas%20Hit)))
    (Variables|Default|SetHas%20Hit true)
    (Game|Damage|ApplyDamage OtherActor (Variables|Default|GetDamage) 0 self)
    (Audio|SpawnSoundatLocation (Variables|Default|GetSoundEffect) (Transformation|GetActorLocation OtherActor) "0, 0, 0" 1.0 1.0 0.0 0 0)
    (Actor|DestroyActor)))

(event EventBeginPlay
  (Audio|PlaySoundatLocation "/Game/Characters/Audio/Frying_Food_sound_effect_Cue.Frying_Food_sound_effect_Cue" (Transformation|GetActorLocation) "0, 0, 0" 1.0 1.0 17.0 0 0 0))

(event Collision|EventActorBeginOverlap
  (params (OtherActor :type Actor%20Object%20Reference)))

(event Collision|EventHit
  (params (MyComp :type Primitive%20Component%20Object%20Reference) (Other :type Actor%20Object%20Reference) (OtherComp :type Primitive%20Component%20Object%20Reference) (bSelfMoved :type Boolean) (HitLocation :type Vector :default "0, 0, 0") (HitNormal :type Vector :default "0, 0, 0") (NormalImpulse :type Vector :default "0, 0, 0") (Hit :type Hit%20Result%20Structure%20%28by%20ref%29))
  (Audio|SpawnSoundatLocation (Variables|Default|GetSoundEffect) HitLocation "0, 0, 0" 1.0 1.0 0.0 0 0)
  (Actor|DestroyActor))

(event EventDeactivateCollision
  (Collision|SetCollisionEnabled (Variables|Default|GetBox) "NoCollision"))

(event EventActivateCollision
  (Collision|SetCollisionProfileName (Variables|Default|GetBox) "OverlapAll" true :!class /Script/Engine.PrimitiveComponent))

(fn ConstructionScript)

(fn ShootProjectile
  (params (Direction :type Vector))
  (bind _item_mesh (Variables|Default|GetItem%20Mesh))
  (bind _launch_vector (CallFunction|GetLaunchVector Direction))
  (CallFunction|ActivateCollision)
  (Collision|SetCollisionEnabled _item_mesh "QueryAndPhysics")
  (Physics|SetSimulatePhysics _item_mesh true)
  (Class|PrimitiveComponent|SetAllPhysicsLinearVelocity _item_mesh _launch_vector false)
  (Class|PrimitiveComponent|SetAllPhysicsAngularVelocityinDegrees _item_mesh _launch_vector false)
  (Variables|Default|SetIsShoot true))

(fn GetLaunchVector
  (params (Direction :type Vector))
  (return (* (Math|Vector|Normalize (Math|Vector|RotateVectorAroundAxis Direction -1e+01 (Math|Vector|RotateVectorAroundAxis Direction 9e+01 "0.000000,0.000000,1.000000"))) (* (/ (Variables|Default|GetBench%20Mark%20Mass) (Variables|Default|GetMass)) 1e+03))))