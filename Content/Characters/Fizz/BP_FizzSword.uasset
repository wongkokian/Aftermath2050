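; BP_FizzSword is the sword Blueprint for the Fizz character, detecting melee hits on Bob.
; ActivateCollision and DeactivateCollision switch its capsule between query-only and no collision, opening and closing the hit window.
; On overlap with a damageable actor of exactly the Bob class, it passes the sweep location to CharRef.TryDealSwordDamage, delegating damage to that character.
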(event OnComponentBeginOverlap(Capsule)
  (params (OverlappedComponent :type Primitive%20Component%20Object%20Reference) (OtherActor :type Actor%20Object%20Reference) (OtherComp :type Primitive%20Component%20Object%20Reference) (OtherBodyIndex :type Integer) (bFromSweep :type Boolean) (SweepResult :type Hit%20Result%20Structure%20%28by%20ref%29))
  (if (and (Variables|/Script/Engine.Actor|GetbCanBeDamaged OtherActor) (== (Utilities|GetClass OtherActor) "/Game/Characters/Bob.Bob_C"))
    (Default|TryDealSwordDamage (Variables|Default|GetCharRef) (.Location (Collision|BreakHitResult SweepResult)))))

(event EventDeactivateCollision
  (Collision|SetCollisionEnabled (Variables|Default|GetCapsule) "NoCollision"))

(event EventActivateCollision
  (Collision|SetCollisionEnabled (Variables|Default|GetCapsule) "QueryOnly"))

(fn ConstructionScript
  (|CallParentFunction))