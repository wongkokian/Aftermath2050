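; BP_Fizz is a sword-wielding boss character that fights Bob, the player.
; Damage updates Bob's boss HUD, asks the controller to enter a second stage below half health, and on death signals level cleared.
; Damage-state events toggle sword and arm collision, with a gate limiting arm overlaps to one hit per opening.
; A Tick-fed gate smoothly yaws Fizz toward Bob, and helper events switch chase and strafe speeds.
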(event OnComponentBeginOverlap(RightArm)
  (params (OverlappedComponent :type Primitive%20Component%20Object%20Reference) (OtherActor :type Actor%20Object%20Reference) (OtherComp :type Primitive%20Component%20Object%20Reference) (OtherBodyIndex :type Integer) (bFromSweep :type Boolean) (SweepResult :type Hit%20Result%20Structure%20%28by%20ref%29))
  ;[1 1 1] Damage
  (if (Utilities|CanHitBob OtherActor)
    (CallFunction|TryDealSwordDamage (.Location (Collision|BreakHitResult SweepResult)))))

(event OnComponentBeginOverlap(LeftArm)
  (params (OverlappedComponent :type Primitive%20Component%20Object%20Reference) (OtherActor :type Actor%20Object%20Reference) (OtherComp :type Primitive%20Component%20Object%20Reference) (OtherBodyIndex :type Integer) (bFromSweep :type Boolean) (SweepResult :type Hit%20Result%20Structure%20%28by%20ref%29))
  ;[1 1 1] Damage
  (if (Utilities|CanHitBob OtherActor)
    (Development|PrintString "Hit by left arm")
    (CallFunction|TryDealSwordDamage (.Location (Collision|BreakHitResult SweepResult)))))

(event Custom|SetChaseSpeed
  (Variables|/Script/Engine.CharacterMovementComponent|SetMaxWalkSpeed (Variables|Character|GetCharacterMovement) (Variables|Default|GetChaseSpeed)))

(event Custom|SetStrafeSpeed
  (Variables|/Script/Engine.CharacterMovementComponent|SetMaxWalkSpeed (Variables|Character|GetCharacterMovement) (Variables|Default|GetStrafeSpeed)))

(event Custom|DisableLeftarmCollision
  ;[1 1 1] Damage
  (Collision|SetCollisionEnabled (Variables|Default|GetLeftArm) "NoCollision"))

(event Custom|DamageStateEnd
  ;[1 1 1] Damage
  (Default|DeactivateCollision (Variables|Default|GetSword))
  (Collision|SetCollisionEnabled (Variables|Default|GetRightArm) "NoCollision")
  (CallFunction|CloseDealDamage))

(event Custom|DamageStateStart
  ;[1 1 1] Damage
  (Default|ActivateCollision (Variables|Default|GetSword))
  (Collision|SetCollisionEnabled (Variables|Default|GetRightArm) "QueryOnly")
  (CallFunction|OpenDealDamage))

(event Custom|TryDealSwordDamage
  (params (HitLocation :type Vector))
  ;[1 1 1] Damage
  (Utilities|FlowControl|Gate true
    (:Exit
      (CallFunction|CloseDealDamage)
      (Game|Damage|ApplyDamage (Variables|Default|GetPlayerRef) (Variables|Default|GetSwordDamage) 0 self)
      (Audio|PlaySoundatLocation "/Game/Characters/Sound/melee_sound.melee_sound" HitLocation "0, 0, 0" 1.0 1.0 0.0 0 0 0))))

(event Custom|OpenDealDamage
  ;[1 1 1] Damage
  (Utilities|FlowControl|Gate true) ; enters at Open
)

(event Custom|CloseDealDamage
  ;[1 1 1] Damage
  (Utilities|FlowControl|Gate true) ; enters at Close
)

(event Custom|RotateToBob
  (Utilities|FlowControl|Gate true) ; enters at Open
)

(event Custom|StopRotateToBob
  (Utilities|FlowControl|Gate true) ; enters at Close
)

(event Custom|EnableLeftarmCollision
  ;[1 1 1] Damage
  (Collision|SetCollisionEnabled (Variables|Default|GetLeftArm) "QueryOnly"))

(event EventBeginPlay
  (Variables|Default|SetAiController (.AsBP%20Fizz%20Controller (Utilities|Casting|CastToBP_FizzController (Pawn|GetController))))
  (Variables|Default|SetPlayerRef (.AsBob (Utilities|Casting|CastToBob (Game|GetPlayerCharacter 0))))
  (Variables|Default|SetAnimBp (.AsFizz%20Anim%20Bp (Utilities|Casting|CastToFizz_AnimBp (Components|SkeletalMesh|GetAnimInstance (Variables|Character|GetMesh)))))
  (CallFunction|SpawnWeapon)
  (Variables|Default|SetInitialHealth (Variables|Default|GetHealth)))

(event EventTick
  (params (DeltaSeconds :type Float%20%28single-precision%29))
  (Utilities|FlowControl|Gate true
    (:Exit
      (Transformation|SetActorRotation self (Math|Interpolation|RInterpTo (Transformation|GetActorRotation) (Math|Rotator|MakeRotator 0.0 0.0 (.yaw (Math|Rotator|FindLookatRotation (Transformation|GetActorLocation) (Transformation|GetActorLocation (Variables|Default|GetPlayerRef))))) DeltaSeconds (Variables|Default|GetRotateSpeed))))))

(event Game|Damage|EventAnyDamage
  (params (Damage :type Float%20%28single-precision%29) (DamageType :type Damage%20Type%20Object%20Reference) (InstigatedBy :type Controller%20Object%20Reference) (DamageCauser :type Actor%20Object%20Reference))
  (CallFunction|PrintDamage DamageCauser Damage)
  (if (> (Variables|Default|GetHealth) 0.0)
    (bind _output_get (Variables|Default|SetHealth (- (Variables|Default|GetHealth) Damage)))
    (bind _asbob (Utilities|Casting|CastToBob (Game|GetPlayerCharacter 0)))
    (bind _output_get_2 (Variables|/Game/HUD/HUD.HUD_C|SetBossHealth (Variables|/Game/Characters/Bob.Bob_C|GetHUD _asbob) _output_get))
    (if (> _output_get_2 0.0)
      (if (Utilities|CanEnterSecondStage)
        (Utilities|FlowControl|DoOnce false
          (:Completed
            (Default|EnterSecondStage (Variables|Default|GetAiController)))))
      (else
        (Default|OnKilled (Variables|Default|GetAiController))
        (Animation|StopAnimMontage 0)
        (Variables|/Game/Characters/Fizz/Fizz_AnimBp.Fizz_AnimBp_C|SetIsAlive (Variables|Default|GetAnimBp) false)
        (CallFunction|DamageStateEnd)
        (CallFunction|CloseDealDamage)
        (CallFunction|StopRotatetoBob)
        (Utilities|FlowControl|Delay 0.2)
        (Collision|SetCollisionEnabled (Variables|Collision|GetCapsuleComponent) "NoCollision")
        (Default|OnLevelCleared (Variables|Default|GetILevelManager))
        (Variables|/Game/HUD/HUD.HUD_C|SetBossBarVisibility (Variables|/Game/Characters/Bob.Bob_C|GetHUD _asbob) "Hidden")
        (Variables|/Game/HUD/HUD.HUD_C|SetBossNameVisibility (Variables|/Game/Characters/Bob.Bob_C|GetHUD _asbob) "Hidden")))))

(event EventHideLockSpot
  ;[1 1 1] Lock Spot
  (Development|SetHiddeninGame (Variables|Default|GetLockSpot) true false))

(event EventShowLockSpot
  ;[1 1 1] Lock Spot
  (Development|SetHiddeninGame (Variables|Default|GetLockSpot) false false))

(fn ConstructionScript)

(fn PrintDamage
  (params (Actor :type Actor%20Object%20Reference) (Damage :type Float%20%28single-precision%29))
  (Development|PrintString (Utilities|String|BuildString(Float) (Utilities|String|ToString(Object) self) " received damage: " Damage (Utilities|String|BuildString(Float) "" " Current health: " (Variables|Default|GetHealth) (Utilities|String|BuildString(Object) "" " Weapon: " Actor)))))

(fn SpawnWeapon
  (bind _returnvalue (Game|SpawnActorfromClass "/Game/Characters/Fizz/BP_FizzSword.BP_FizzSword_C" (Transformation|GetSocketTransform (Variables|Character|GetMesh) "WeaponSocket" "RTS_World") "Undefined" 0 0))
  (Transformation|AttachComponentToComponent _returnvalue (Variables|Character|GetMesh) "WeaponSocket" "SnapToTarget" "SnapToTarget" "SnapToTarget" true)
  (bind _output_get (Variables|Default|SetSword _returnvalue))
  (Variables|/Game/Characters/Fizz/BP_FizzSword.BP_FizzSword_C|SetCharRef _output_get self))

(fn IsAlive
  (return (> (Variables|Default|GetHealth) 0.0)))