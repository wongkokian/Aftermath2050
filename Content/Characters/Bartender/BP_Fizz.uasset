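; BP_Fizz is an AI-controlled, sword-wielding character with health, driven by BP_FizzController.
; On BeginPlay it caches that controller, then spawns a BP_FizzSword and attaches it to the mesh's WeaponSocket.
; AnyDamage prints debug info and reduces Health, calling OnKilled on the controller when it runs out.
; Events toggle the LockSpot marker's visibility and switch movement between chase and strafe speeds.
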(event Custom|SetChaseSpeed
  (Variables|/Script/Engine.CharacterMovementComponent|SetMaxWalkSpeed (Variables|Character|GetCharacterMovement) (Variables|Default|GetChaseSpeed)))

(event Custom|SetStrafeSpeed
  (Variables|/Script/Engine.CharacterMovementComponent|SetMaxWalkSpeed (Variables|Character|GetCharacterMovement) (Variables|Default|GetStrafeSpeed)))

(event EventBeginPlay
  (bind _asbp_fizz_controller (Utilities|Casting|CastToBP_FizzController (Pawn|GetController)))
  (Variables|Default|SetAiController _asbp_fizz_controller)
  (CallFunction|SpawnWeapon))

(event Game|Damage|EventAnyDamage
  (params (Damage :type Float%20%28single-precision%29) (DamageType :type Damage%20Type%20Object%20Reference) (InstigatedBy :type Controller%20Object%20Reference) (DamageCauser :type Actor%20Object%20Reference))
  (CallFunction|PrintDamage DamageCauser Damage)
  (if (> (Variables|Default|GetHealth) 0.0)
    (bind _output_get (Variables|Default|SetHealth (- (Variables|Default|GetHealth) Damage)))
    (if (not (> _output_get 0.0))
      (Default|OnKilled (Variables|Default|GetAiController)))))

(event EventHideLockSpot
  (Development|SetHiddeninGame (Variables|Default|GetLockSpot) true false))

(event EventShowLockSpot
  (Development|SetHiddeninGame (Variables|Default|GetLockSpot) false false))

(fn ConstructionScript)

(fn PrintDamage
  (params (Actor :type Actor%20Object%20Reference) (Damage :type Float%20%28single-precision%29))
  (Development|PrintString (Utilities|String|BuildString(Float) (Utilities|String|ToString(Object) self) " received damage: " Damage (Utilities|String|BuildString(Float) "" " Current health: " (Variables|Default|GetHealth) (Utilities|String|BuildString(Object) "" " Weapon: " Actor)))))

(fn SpawnWeapon
  (bind _returnvalue (Game|SpawnActorfromClass "/Game/Characters/Bartender/BP_FizzSword.BP_FizzSword_C" (Transformation|GetSocketTransform (Variables|Character|GetMesh) "WeaponSocket" "RTS_World") "Undefined" 0 0))
  (Transformation|AttachComponentToComponent _returnvalue (Variables|Character|GetMesh) "WeaponSocket" "SnapToTarget" "SnapToTarget" "SnapToTarget" true)
  (Variables|Default|SetSword _returnvalue))

(fn IsAlive
  (return (> (Variables|Default|GetHealth) 0.0)))