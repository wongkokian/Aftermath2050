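; Ranged zombie enemy that holds a random projectile weapon in its hand socket, throws it at the player and spawns a new one after a delay.
; Each tick a line trace tells its AI controller whether the view to the player is blocked.
; Damage updates a health bar widget and triggers hit knockback or death with a random speed or medkit drop.
; It also provides a lock-on marker and a slow-motion kill cam that picks an unobstructed camera.
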(event OnComponentBeginOverlap(Sphere)
  (params (OverlappedComponent :type Primitive%20Component%20Object%20Reference) (OtherActor :type Actor%20Object%20Reference) (OtherComp :type Primitive%20Component%20Object%20Reference) (OtherBodyIndex :type Integer) (bFromSweep :type Boolean) (SweepResult :type Hit%20Result%20Structure%20%28by%20ref%29))
  (Utilities|Casting|CastToBob OtherActor)
  (Rendering|SetVisibility (Variables|Default|GetWidget) true false))

(event OnComponentEndOverlap(Sphere)
  (params (OverlappedComponent :type Primitive%20Component%20Object%20Reference) (OtherActor :type Actor%20Object%20Reference) (OtherComp :type Primitive%20Component%20Object%20Reference) (OtherBodyIndex :type Integer))
  (Utilities|Casting|CastToBob OtherActor)
  (Rendering|SetVisibility (Variables|Default|GetWidget) false false))

(event Custom|SetSpeed
  (params (Speed :type Float%20%28single-precision%29))
  (Variables|/Script/Engine.CharacterMovementComponent|SetMaxWalkSpeed (Variables|Character|GetCharacterMovement) Speed))

(event Custom|Shoot
  (Utilities|ShootProjectile)
  (Utilities|FlowControl|Delay 2.5)
  (CallFunction|SpawnWeapon (Utilities|RandomWeapon)))

(event EventBeginPlay
  (CallFunction|Init)
  (CallFunction|SpawnWeapon (Utilities|RandomWeapon))
  (Variables|Default|SetAttack%20Range (Variables|/Game/Characters/Weapons/EnemyProjectile.EnemyProjectile_C|GetAttackRange (Variables|Default|GetHeld%20Item)))
  (bind _asenemy_healthbar_widget (Utilities|Casting|CastToEnemyHealthbar_Widget (UserInterface|GetUserWidgetObject (Variables|Default|GetWidget))))
  (bind _output_get (Variables|Default|SetEnemyHealthWidget _asenemy_healthbar_widget))
  (Variables|/Game/EnemyHealthbar/EnemyHealthbar_Widget.EnemyHealthbar_Widget_C|SetMax%20Health _output_get (Variables|Default|GetHealth))
  (Variables|/Game/EnemyHealthbar/EnemyHealthbar_Widget.EnemyHealthbar_Widget_C|SetHealth _output_get (Variables|Default|GetHealth)))

(event Game|Damage|EventAnyDamage
  (params (Damage :type Float%20%28single-precision%29) (DamageType :type Damage%20Type%20Object%20Reference) (InstigatedBy :type Controller%20Object%20Reference) (DamageCauser :type Actor%20Object%20Reference))
  (bind _returnvalue (Transformation|GetActorLocation))
  (bind _aicontroller (Variables|Default|GetAiController))
  (bind _returnvalue_2 (+ _returnvalue "0, 0,50.000000"))
  (bind _returnvalue_3 (Math|Conversions|ToTransform(Vector) _returnvalue_2))
  (bind _output_get (Variables|Default|SetHealth (- (Variables|Default|GetHealth) Damage)))
  (Variables|/Game/EnemyHealthbar/EnemyHealthbar_Widget.EnemyHealthbar_Widget_C|SetHealth (Variables|Default|GetEnemyHealthWidget) _output_get)
  (Rendering|SetVisibility (Variables|Default|GetWidget) true false)
  (if (> (Variables|Default|GetHealth) 0.0)
    (Default|OnHit _aicontroller)
    (Animation|PlayAnimMontage "/Game/Characters/Animations/Zombie_Reaction_Hit_Short.Zombie_Reaction_Hit_Short" 1.0 "None")
    (Physics|AddImpulse (Variables|Character|GetCharacterMovement) (Utilities|GetHitImpulse (Game|Player|GetPlayerPawn 0) (Variables|Default|GetHitImpulse)) true)
    (else
      (Default|OnKilled _aicontroller)
      (Variables|/Game/Characters/Animations/ThrowZombie_AnimBP.ThrowZombie_AnimBP_C|SetIsAlive (Variables|Default|GetAnimBP) false)
      (switch int (Math|Random|RandomInteger 3)
        (:0
          (Game|SpawnActorfromClass "/Game/Buffs/BP_Speed.BP_Speed_C" _returnvalue_3 "Undefined" 0 0))
        (:1
          (Game|SpawnActorfromClass "/Game/Buffs/BP_Medkit.BP_Medkit_C" _returnvalue_3 "Undefined" 0 0))))))

(event EventKillCam
  (CallFunction|ChooseCamera)
  (CallFunction|ChangeCamera)
  (Utilities|Time|SetGlobalTimeDilation 0.5)
  (Utilities|FlowControl|Delay 2.0)
  (Utilities|Time|SetGlobalTimeDilation 1.0)
  (CallFunction|ChangeCameraBack))

(event EventShowLockSpot
  (Development|SetHiddeninGame (Variables|Default|GetLockSpot) false false))

(event EventHideLockSpot
  (Development|SetHiddeninGame (Variables|Default|GetLockSpot) true false))

(event EventTick
  (params (DeltaSeconds :type Float%20%28single-precision%29))
  (bind _aicontroller (Variables|Default|GetAiController))
  (bind _isblock (CallFunction|IsBlock))
  (if _isblock
    (Default|OnBlocked _aicontroller)
    (else
      (Default|OnNotBlocked _aicontroller))))

(event Collision|EventActorBeginOverlap
  (params (OtherActor :type Actor%20Object%20Reference)))

(fn ConstructionScript)

(fn Init
  (bind _asthrow_zombie_anim_bp (Utilities|Casting|CastToThrowZombie_AnimBP (Components|SkeletalMesh|GetAnimInstance (Variables|Character|GetMesh))))
  (Variables|Default|SetAnimBP _asthrow_zombie_anim_bp)
  (bind _asbp_throw_zombie_controller (Utilities|Casting|CastToBP_ThrowZombieController (Pawn|GetController)))
  (Variables|Default|SetAiController _asbp_throw_zombie_controller))

(fn IsBlock
  (bind _returnvalue (Collision|LineTraceByChannel (Transformation|GetActorLocation) (Transformation|GetWorldLocation (Variables|/Script/Engine.Character|GetCapsuleComponent (Game|GetPlayerCharacter 0))) "TraceTypeQuery1" false 0 "None"))
  (return _returnvalue))

(fn SpawnWeapon
  (params (Weapon%20Type :type Actor%20Class%20Reference))
  (bind _returnvalue (Game|SpawnActorfromClass Weapon%20Type (Transformation|GetSocketTransform (Variables|Character|GetMesh) "WeaponSocket" "RTS_World") "AlwaysSpawn" 0 0))
  (bind _asenemy_projectile (Utilities|Casting|CastToEnemyProjectile _returnvalue))
  (Class|IWeapon|DeactivateCollision(Message) _asenemy_projectile)
  (Transformation|AttachComponentToComponent _asenemy_projectile (Variables|Character|GetMesh) "WeaponSocket" "SnapToTarget" "SnapToTarget" "SnapToTarget" true)
  (Variables|Default|SetHeld%20Item _asenemy_projectile)
  (Variables|Default|SetIsHolding true))

(fn ChangeCamera
  (Game|Player|SetViewTargetwithBlend (Game|GetPlayerController 0) (Components|GetOwner (Variables|Default|GetCamera)) 0.0 "VTBlend_Linear" 0.0 false))

(fn ChangeCameraBack
  (bind _asbob (Utilities|Casting|CastToBob (Game|GetPlayerCharacter 0)))
  (Game|Player|SetViewTargetwithBlend (Game|GetPlayerController 0) (Components|GetOwner (Variables|/Game/Characters/Bob.Bob_C|GetFollowCamera _asbob)) 0.0 "VTBlend_Linear" 0.0 false))

(fn ChooseCamera
  (bind _camera (Variables|Default|GetCamera))
  (bind _camera1 (Variables|Default|GetCamera1))
  (bind _returnvalue (Collision|LineTraceByChannel (Transformation|GetWorldLocation (Variables|Default|GetCamera)) (Transformation|GetWorldLocation (Variables|/Script/Engine.Character|GetCapsuleComponent (Game|GetPlayerCharacter 0))) "TraceTypeQuery1" false 0 "None"))
  (if _returnvalue
    (Components|Activation|SetActive _camera false true)
    (Components|Activation|SetActive _camera1 true false)
    (else
      (Components|Activation|SetActive _camera true false)
      (Components|Activation|SetActive _camera1 false true))))

(fn IsAlive
  (return (> (Variables|Default|GetHealth) 0.0)))