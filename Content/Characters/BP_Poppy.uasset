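; Poppy is an NPC character who shows speech text through an ActivateDialogue event and can hand the player a coffee.
; ActivateSpeech either spawns BP_Coffee beside her or shows a random line and increments a counter.
; CanSpawnCoffee gates the gift, though its one-time, low-health, counter-weighted chance logic appears unconnected.
; Leaving her sphere hides the text, while Bob entering it only reaches an empty DoOnce.
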(event OnComponentBeginOverlap(Sphere)
  (params (OverlappedComponent :type Primitive%20Component%20Object%20Reference) (OtherActor :type Actor%20Object%20Reference) (OtherComp :type Primitive%20Component%20Object%20Reference) (OtherBodyIndex :type Integer) (bFromSweep :type Boolean) (SweepResult :type Hit%20Result%20Structure%20%28by%20ref%29))
  (if (== (Utilities|GetClass OtherActor) "/Game/Characters/Bob.Bob_C")
    (Utilities|FlowControl|DoOnce false)))

(event OnComponentEndOverlap(Sphere)
  (params (OverlappedComponent :type Primitive%20Component%20Object%20Reference) (OtherActor :type Actor%20Object%20Reference) (OtherComp :type Primitive%20Component%20Object%20Reference) (OtherBodyIndex :type Integer))
  (CallFunction|DeactivateSpeech))

(event EventBeginPlay)

(event Collision|EventActorBeginOverlap
  (params (OtherActor :type Actor%20Object%20Reference)))

(event EventTick
  (params (DeltaSeconds :type Float%20%28single-precision%29)))

(event EventActivateDialogue
  (CallFunction|ActivateSpeech))

(fn ConstructionScript)

(fn ActivateSpeech
  (bind __hello (Variables|Default|Get%20Hello))
  (bind _capsulecomponent (Variables|Collision|GetCapsuleComponent))
  (Rendering|SetVisibility __hello true false)
  (if (Utilities|CanSpawnCoffee)
    (Rendering|Components|TextRender|SetText __hello (Utilities|Text|MakeLiteralText "Boi you look tired. Here, have a cup of coffee!"))
    (Game|SpawnActorfromClass "/Game/Buffs/BP_Coffee.BP_Coffee_C" (Math|Conversions|ToTransform(Vector) (+ (Transformation|GetWorldLocation _capsulecomponent) (* (Math|Vector|RotateVectorAroundAxis (Math|Vector|GetForwardVector _capsulecomponent) 9e+01 "0, 0,1.000000") 1e+02))) "Undefined" 0 0)
    (Variables|Default|SetHasSpawnedCoffee true)
    (else
      (Rendering|Components|TextRender|SetText __hello (Utilities|Text|ToText(String) (.OutItem (Utilities|Array|Random (Variables|Default|Gettext%20array)))))
      (Math|Integer|IncrementInt (Variables|Default|Getcounter)))))

(fn DeactivateSpeech
  (Rendering|SetVisibility (Variables|Default|Get%20Hello) false false))