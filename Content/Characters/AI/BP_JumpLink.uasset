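; Smart nav link that makes AI characters jump when they reach it during pathfinding.
; On SmartLinkReached, any agent that casts to Character is treated as jumpable and passed to AiJump.
; AiJump turns the character horizontally toward the world origin, not the link's destination, then launches it that way at max movement speed.
; Upward velocity is slightly above its JumpZVelocity, and the launch overrides existing velocity.
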(event Collision|EventActorBeginOverlap
  (params (OtherActor :type Actor%20Object%20Reference)))

(event EventTick
  (params (DeltaSeconds :type Float%20%28single-precision%29)))

(event EventSmartLinkReached
  (params (Agent :type Actor%20Object%20Reference) (Destination :type Vector%20%28by%20ref%29 :default "0, 0, 0"))
  (bind (_character _jumpable) (CallFunction|IsJumpable Agent))
  (if _jumpable
    (CallFunction|AiJump _character)))

(fn ConstructionScript)

(fn IsJumpable
  (params (Zombie :type Actor%20Object%20Reference))
  (bind _ascharacter (Utilities|Casting|CastToCharacter Zombie)
    (:then
      (return _ascharacter true))
    (:CastFailed
      (return 0 false))))

(fn AiJump
  (params (Character :type Character%20Object%20Reference))
  (bind _returnvalue (Transformation|GetActorLocation Character))
  (bind _charactermovement (Variables|/Script/Engine.Character|GetCharacterMovement Character))
  (bind _returnvalue_2 (- "0, 0, 0" _returnvalue))
  (bind _returnvalue_3 (Math|Conversions|ToVector2D(Vector) _returnvalue_2))
  (bind _returnvalue_4 (Math|Conversions|ToVector(Vector2D) _returnvalue_3))
  (Transformation|SetActorRotation Character (Math|Conversions|RotationFromXVector _returnvalue_4))
  (Character|LaunchCharacter Character (+ (* (Math|Vector|Normalize _returnvalue_4) (Class|MovementComponent|GetMaxSpeed _charactermovement)) (Math|Vector|MakeVector 0.0 0.0 (+ (Variables|/Script/Engine.CharacterMovementComponent|GetJumpZVelocity _charactermovement) 5e+01))) true true))