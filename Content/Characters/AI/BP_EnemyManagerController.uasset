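; AI controller that acts as the stage's enemy manager, tracking spawned zombies and reporting when the level is cleared.
; BeginPlay runs the BT_EnemyManager behavior tree and calls OnBobEnters, which writes itself to the Blackboard, then after a short delay the player and alive flag.
; SpawnZombies fills the Zombies array from Locations using GetRandomZombieType.
; RemoveEnemy shrinks that array and calls OnLevelCleared on the level Blueprint once it empties.
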(event Custom|OnBobEnters
  ;[1 1 1] Assign self as the EnemyManager in blackboard BB_stage
  (AI|Components|Blackboard|SetValueasObject (Variables|Default|GetBlackboard) (Utilities|Name|MakeLiteralName "EnemyManager") self)
  (Utilities|FlowControl|Delay 0.2)
  (AI|Components|Blackboard|SetValueasObject (Variables|Default|GetBlackboard) (Utilities|Name|MakeLiteralName "PlayerActor") (Game|GetPlayerCharacter 0))
  (AI|Components|Blackboard|SetValueasBool (Variables|Default|GetBlackboard) (Utilities|Name|MakeLiteralName "IsPlayerAlive") true))

(event Custom|RemoveEnemy
  (params (ToRemove :type Actor%20Object%20Reference))
  (bind _zombies (Variables|Default|GetZombies))
  (bind _returnvalue (Utilities|Array|RemoveItem _zombies ToRemove))
  (if _returnvalue
    (if (== (Utilities|Array|Length _zombies) 0)
      (Default|OnLevelCleared (Variables|Default|GetLevelBp)))))

(event EventBeginPlay
  (AI|RunBehaviorTree "/Game/Characters/AI/BT_EnemyManager.BT_EnemyManager")
  ;[1 1 1] Used in test stage
  (CallFunction|OnBobEnters))

(fn ConstructionScript)

(fn SpawnZombies
  (for _array_element (Variables|Default|GetLocations)
    (bind _returnvalue (Game|SpawnActorfromClass (Utilities|GetRandomZombieType) (Math|Transform|MakeTransform _array_element) "Undefined" 0 0))
    (Utilities|Array|Add (Variables|Default|GetZombies) _returnvalue)))