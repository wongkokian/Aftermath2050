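; Melee zombie enemy character that spawns with a bat attached to its weapon socket and takes its attack range from it.
; Damage lowers health, then either triggers a hit reaction with knockback relative to the player or, at zero health, notifies the AI controller and AnimBP of death.
; Repeated hits within a time window grant temporary hyperarmour, which suppresses reactions and lights an emissive material until a delay resets it.
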(event Custom|SetSpeed
  (params (Speed :type Float%20%28single-precision%29))
  (Variables|/Script/Engine.CharacterMovementComponent|SetMaxWalkSpeed (Variables|Character|GetCharacterMovement) Speed))

(event Custom|HyperarmourCountdown
  (Utilities|FlowControl|DoOnce false :!label _label
    (:Completed
      (Rendering|Material|SetScalarParameterValueonMaterials (Variables|Character|GetMesh) "EmissiveColor" 1.0)
      (Utilities|FlowControl|Delay (Variables|Default|GetHyperarmourTime))
      (CallFunction|ResetHitCount)
      (Variables|Default|SetIsHyperarmour false)
      (Rendering|Material|SetScalarParameterValueonMaterials (Variables|Character|GetMesh) "EmissiveColor" 0.0)
      (goto _label Reset))))

(event EventBeginPlay
  (CallFunction|Init)
  (CallFunction|SpawnWeapon "/Game/Characters/Weapons/BP_EnemyBat.BP_EnemyBat_C")
  (bind _asenemy_sword_weapon (Utilities|Casting|CastToEnemySwordWeapon (Variables|Default|GetHeld%20Item)))
  (Variables|Default|SetAttackRange (Variables|/Game/Characters/Weapons/EnemySwordWeapon.EnemySwordWeapon_C|GetAttackRange _asenemy_sword_weapon)))

(event Game|Damage|EventAnyDamage
  (params (Damage :type Float%20%28single-precision%29) (DamageType :type Damage%20Type%20Object%20Reference) (InstigatedBy :type Controller%20Object%20Reference) (DamageCauser :type Actor%20Object%20Reference))
  (if (> (Variables|Default|GetHealth) 0.0)
    (Variables|Default|SetHealth (- (Variables|Default|GetHealth) Damage))
    (if (Variables|Default|GetPrintDamage)
      _
      (else
        _))
    (CallFunction|SetHitCount)
    (if (> (Variables|Default|GetHealth) 0.0)
      (if (Variables|Default|GetIsHyperarmour)
        (CallFunction|HyperarmourCountdown)
        (else
          (Default|OnHit (Variables|Default|GetAiController))
          (Animation|StopAnimMontage "/Game/Characters/Animations/Zombie_MeleeUpper_Montage.Zombie_MeleeUpper_Montage")
          (Animation|PlayAnimMontage "/Game/Characters/Animations/Zombie_Reaction_Hit_Short.Zombie_Reaction_Hit_Short" 1.0 "None")
          (Physics|AddImpulse (Variables|Character|GetCharacterMovement) (Utilities|GetHitImpulse (Game|Player|GetPlayerPawn 0) (Variables|Default|GetHitImpulse)) true)))
      (else
        (Animation|StopAnimMontage 0)
        (Default|OnKilled (Variables|Default|GetAiController))
        (Variables|/Game/Characters/Animations/MeleeZombie_AnimBP.MeleeZombie_AnimBP_C|SetIsAlive (Variables|Default|GetAnimBP) false)))))

(fn ConstructionScript)

(fn Init
  (bind _asmelee_zombie_anim_bp (Utilities|Casting|CastToMeleeZombie_AnimBP (Components|SkeletalMesh|GetAnimInstance (Variables|Character|GetMesh))))
  (Variables|Default|SetAnimBP _asmelee_zombie_anim_bp)
  (bind _asbp_melee_zombie_controller (Utilities|Casting|CastToBP_MeleeZombieController (Pawn|GetController)))
  (Variables|Default|SetAiController _asbp_melee_zombie_controller))

(fn SetHitCount
  (bind _returnvalue (Actor|GetGameTimeSinceCreation))
  (if (not (Variables|Default|GetIsHyperarmour))
    (if (> (- _returnvalue (Variables|Default|GetHitTime)) (Variables|Default|GetResetTime))
      (CallFunction|ResetHitCount)
      (Variables|Default|SetHitTime _returnvalue))
    (bind _result (Math|Integer|IncrementInt (Variables|Default|GetHitCount))
      (:%20%20
        (if (not (< _result (Variables|Default|GetHitLimit)))
          (Variables|Default|SetIsHyperarmour true))))))

(fn ResetHitCount
  (Variables|Default|SetHitTime 0.0)
  (Variables|Default|SetHitCount 0))

(fn SpawnWeapon
  (params (WeaponType :type Actor%20Class%20Reference))
  (bind _returnvalue (Game|SpawnActorfromClass WeaponType (Transformation|GetSocketTransform (Variables|Character|GetMesh) "WeaponSocket" "RTS_World") "Undefined" 0 0))
  (Transformation|AttachComponentToComponent _returnvalue (Variables|Character|GetMesh) "WeaponSocket" "SnapToTarget" "SnapToTarget" "SnapToTarget" true)
  (Variables|Default|SetHeld%20Item _returnvalue))

(fn DropWeapon
  (bind _held_item (Variables|Default|GetHeld%20Item))
  (bind _asenemy_sword_weapon (Utilities|Casting|CastToEnemySwordWeapon _held_item))
  (Default|SpawnBobWeapon _asenemy_sword_weapon)
  (Actor|DestroyActor _held_item))