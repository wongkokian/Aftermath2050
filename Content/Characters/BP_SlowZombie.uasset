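; BP_SlowZombie is a slow zombie enemy character with health, hit reactions and death.
; On BeginPlay it caches its anim Blueprint and AI controller.
; Damage lowers health, then either notifies the controller, plays a hit montage and applies an impulse, or reports death and clears the anim Blueprint's alive flag.
; It also exposes events to damage a target and set walk speed.
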(event Custom|OnHit
  (Animation|PlayAnimMontage 0 1.0 "None"))

(event Custom|OnKilled)

(event Custom|Set%20Speed
  (params (Speed :type Float%20%28single-precision%29))
  (Variables|/Script/Engine.CharacterMovementComponent|SetMaxWalkSpeed (Variables|Character|GetCharacterMovement) Speed))

(event Custom|Attack%20Player
  (params (Damaged :type Bob%20Object%20Reference))
  (Game|Damage|ApplyDamage Damaged 1e+01 0 self))

(event EventBeginPlay
  (bind _asslow_zombie_anim_bp (Utilities|Casting|CastToSlowZombie_AnimBP (Components|SkeletalMesh|GetAnimInstance (Variables|Character|GetMesh)))
    (:then
      (Variables|Default|SetAnimaBP _asslow_zombie_anim_bp)
      (bind _asbp_slow_zombie_controller (Utilities|Casting|CastToBP_SlowZombieController (Pawn|GetController))
        (:then
          (Variables|Default|SetAiController _asbp_slow_zombie_controller))
        (:CastFailed
          (Development|PrintString "cast failed: zombie controller"))))
    (:CastFailed
      (Development|PrintString "cast failed: zombie anim bp "))))

(event Game|Damage|EventAnyDamage
  (params (Damage :type Float%20%28single-precision%29) (DamageType :type Damage%20Type%20Object%20Reference) (InstigatedBy :type Controller%20Object%20Reference) (DamageCauser :type Actor%20Object%20Reference))
  (bind _aicontroller (Variables|Default|GetAiController))
  (Variables|Default|SetHealth (- (Variables|Default|GetHealth) Damage))
  (Development|PrintString (Utilities|GetDamageString Damage))
  (if (> (Variables|Default|GetHealth) 0.0)
    (Default|OnHit _aicontroller)
    (Animation|PlayAnimMontage "/Game/Characters/Animations/Zombie_Reaction_Hit_Short.Zombie_Reaction_Hit_Short" 1.0 "None")
    (Physics|AddImpulse (Variables|Character|GetCharacterMovement) (Utilities|GetHitImpulse (Game|Player|GetPlayerPawn 0) (Variables|Default|GetHitImpulse)) true)
    (else
      (Default|OnKilled _aicontroller)
      (Variables|/Game/Characters/Animations/SlowZombie_AnimBP.SlowZombie_AnimBP_C|SetIsAlive (Variables|Default|GetAnimaBP) false))))

(fn ConstructionScript)