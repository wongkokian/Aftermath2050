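; BP_InteractionFarmer is a gaze-and-click interactor that lets the player tell objects in the world to grow.
; Each Tick it line-traces along the VR camera's forward vector and moves a material billboard to the hit point as a reticle, or to the world origin on a miss.
; Left mouse click repeats the trace with debug drawing and sends GrowMessage to the hit actor.
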(event EventBeginPlay)

(event Collision|EventActorBeginOverlap
  (params (OtherActor :type Actor%20Object%20Reference)))

(event EventTick
  (params (DeltaSeconds :type Float%20%28single-precision%29))
  (bind _materialbillboard (Variables|Default|GetMaterialBillboard))
  (bind (_location _forward_vector) (CallFunction|GetPlayerVRCameraProperties))
  (bind (_outhit _returnvalue) (Collision|LineTraceByChannel _location (+ _location (* _forward_vector 1e+04) "") "TraceTypeQuery1" false 0 "None"))
  (if _returnvalue
    (Transformation|SetWorldLocation _materialbillboard (.Location (Collision|BreakHitResult _outhit)) false false)
    (else
      (Transformation|SetWorldLocation _materialbillboard "0, 0, 0" false false))))

(event Input|MouseEvents|LeftMouseButton
  (params (Key :type Key%20Structure :default "None"))
  (:Pressed
    (bind (_location _forward_vector) (CallFunction|GetPlayerVRCameraProperties))
    (bind (_outhit _returnvalue) (Collision|LineTraceByChannel _location (+ _location (* _forward_vector 1e+04)) "TraceTypeQuery1" false 0 "ForDuration"))
    (if _returnvalue
      (Class|GrowInterface|Grow(Message) (.HitActor (Collision|BreakHitResult _outhit))))))

(fn ConstructionScript)